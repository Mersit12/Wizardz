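; BP_Campfire is a campfire actor that regenerates the player's health while the character is inside its sphere.
; Entering caches the character, clears its health-change animation, sets a sound and starts a one-second delay loop that spawns healing Niagara effects and raises Health through the attribute component.
; The loop stops at full health or once an exit clears the Active flag, which also restores the hurt montage.
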(event OnComponentBeginOverlap(Sphere)
  (params (OverlappedComponent :type Primitive%20Component%20Object%20Reference) (OtherActor :type Actor%20Object%20Reference) (OtherComp :type Primitive%20Component%20Object%20Reference) (OtherBodyIndex :type Integer) (bFromSweep :type Boolean) (SweepResult :type Hit%20Result%20Structure%20%28by%20ref%29))
  (bind _asbp_third_person_character (Utilities|Casting|CastToBP_ThirdPersonCharacter OtherActor))
  (bind _output_get (Variables|Default|SetPlayerREF _asbp_third_person_character))
  (Variables|/Game/PlayerCharacter/ThirdPerson/Blueprints/BP_ThirdPersonCharacter.BP_ThirdPersonCharacter_C|SetHealthChangeAnim _asbp_third_person_character 0)
  (Variables|/Game/PlayerCharacter/ThirdPerson/Blueprints/BP_ThirdPersonCharacter.BP_ThirdPersonCharacter_C|SetHealthChangeSound _asbp_third_person_character "/Engine/VREditor/Sounds/UI/Enter_Play.Enter_Play")
  (Variables|Default|SetActive true)
  (CallFunction|HealthRegen (Variables|/Game/PlayerCharacter/ThirdPerson/Blueprints/BP_ThirdPersonCharacter.BP_ThirdPersonCharacter_C|GetBPC_Attributes _output_get)))

(event OnComponentEndOverlap(Sphere)
  (params (OverlappedComponent :type Primitive%20Component%20Object%20Reference) (OtherActor :type Actor%20Object%20Reference) (OtherComp :type Primitive%20Component%20Object%20Reference) (OtherBodyIndex :type Integer))
  (bind _asbp_third_person_character (Utilities|Casting|CastToBP_ThirdPersonCharacter OtherActor))
  (Variables|Default|SetActive false)
  (Variables|/Game/PlayerCharacter/ThirdPerson/Blueprints/BP_ThirdPersonCharacter.BP_ThirdPersonCharacter_C|SetHealthChangeAnim _asbp_third_person_character "/Game/PlayerCharacter/Animations/Montages/Hurt/UE5_WZ_Hurt_Variations_01_Seq_Montage.UE5_WZ_Hurt_Variations_01_Seq_Montage"))

(event Custom|HealthRegen
  (params (Target :type BPC%20Attributes%20Object%20Reference))
  (if (Variables|Default|GetActive) :!label _label
    (bind _returnvalue (Niagara|SpawnSystematLocation "/Game/VFX/WizardSpellsPack/sA_Megapack_v1/sA_PickupSet_1/Fx/NiagaraSystems/NS_Healing_3.NS_Healing_3" (Transformation|GetActorLocation (Game|GetPlayerCharacter 0))))
    (Variables|Default|SetParticleREF _returnvalue)
    (Default|ChangeAttribute Target "(TagName=\"Attribute.Health\")" 2.0 "NewEnumerator1" (Utilities|Struct|MakeS_Origin (Game|GetPlayerCharacter 0) (Game|GetPlayerController 0)))
    (Utilities|FlowControl|Delay 1.0)
    (if (not (== (.BaseValue (Utilities|Struct|BreakS_Attribute (Variables|/Game/Blueprints/Attributes/BPC_Attributes.BPC_Attributes_C|GetHealth (Variables|/Game/PlayerCharacter/ThirdPerson/Blueprints/BP_ThirdPersonCharacter.BP_ThirdPersonCharacter_C|GetBPC_Attributes (Variables|Default|GetPlayerREF))))) 1e+02))
      (goto _label))))

(event EventBeginPlay)

(event Collision|EventActorBeginOverlap
  (params (OtherActor :type Actor%20Object%20Reference)))

(event EventTick
  (params (DeltaSeconds :type Float%20%28single-precision%29)))

(fn ConstructionScript)
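; Staff weapon Blueprint that defines its damage locations and shows floating damage numbers.
; GetDamageLocations returns one pair of points from the static mesh's A and B sockets.
; MakeDamageNumbers spawns one NS_DamageNumbers Niagara system per digit, yawed to player 0's control rotation, and sets its digit texture parameter.
; Digits are spaced along local Y by an accumulating TextOffset, which this function never resets.
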(event EventBeginPlay
  (|CallParentFunction))

(event Collision|EventActorBeginOverlap
  (params (OtherActor :type Actor%20Object%20Reference)))

(event EventTick
  (params (DeltaSeconds :type Float%20%28single-precision%29)))

(fn ConstructionScript
  (|CallParentFunction))

(fn GetDamageLocations
  (bind _staticmesh (Variables|Default|GetStaticMesh))
  (return (Utilities|Array|MakeArray (Utilities|Struct|MakeS_DamageLocations (Transformation|GetSocketLocation _staticmesh "A") (Transformation|GetSocketLocation _staticmesh "B")))))

(fn MakeDamageNumbers
  (params (Location :type Vector) (DamageAmount :type Integer))
  (for _array_element (Utilities|String|GetCharacterArrayfromString (Utilities|String|ToString(Integer) DamageAmount))
    (bind _returnvalue (Niagara|SpawnSystematLocation "/Game/Blueprints/Abilities/NS_DamageNumbers.NS_DamageNumbers" Location (Math|Rotator|MakeRotator 0.0 1.8e+02 (.yaw (Pawn|GetControlRotation (Game|GetPlayerController 0) :!class /Script/Engine.Controller)))))
    (bind _output_get (Variables|Default|SetDigitSystem _returnvalue))
    (Transformation|AddLocalOffset _output_get (Math|Vector|MakeVector 0.0 (Variables|Default|GetTextOffset) 0.0) false false)
    (Variables|Default|SetTextOffset (+ (Variables|Default|GetTextOffset) 25.0))
    (switch string _array_element
      (:0
        (Niagara|SetTextureObject (Variables|Default|GetDigitSystem) "user.Digit" "/Game/VFX/DamageDigits/0.0"))
      (:1
        (Niagara|SetTextureObject (Variables|Default|GetDigitSystem) "user.Digit" "/Game/VFX/DamageDigits/1.1"))
      (:2
        (Niagara|SetTextureObject (Variables|Default|GetDigitSystem) "user.Digit" "/Game/VFX/DamageDigits/2.2"))
      (:3
        (Niagara|SetTextureObject (Variables|Default|GetDigitSystem) "user.Digit" "/Game/VFX/DamageDigits/3.3"))
      (:4
        (Niagara|SetTextureObject (Variables|Default|GetDigitSystem) "user.Digit" "/Game/VFX/DamageDigits/4.4"))
      (:5
        (Niagara|SetTextureObject (Variables|Default|GetDigitSystem) "user.Digit" "/Game/VFX/DamageDigits/5.5"))
      (:6
        (Niagara|SetTextureObject (Variables|Default|GetDigitSystem) "user.Digit" "/Game/VFX/DamageDigits/6.6"))
      (:7
        (Niagara|SetTextureObject (Variables|Default|GetDigitSystem) "user.Digit" "/Game/VFX/DamageDigits/7.7"))
      (:8
        (Niagara|SetTextureObject (Variables|Default|GetDigitSystem) "user.Digit" "/Game/VFX/DamageDigits/8.8"))
      (:9
        (Niagara|SetTextureObject (Variables|Default|GetDigitSystem) "user.Digit" "/Game/VFX/DamageDigits/9.9")))))
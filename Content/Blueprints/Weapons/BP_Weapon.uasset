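; BP_Weapon is a weapon actor that levels through its own XP component and scales its damage by level.
; On BeginPlay it binds to its owner's XP component and awards itself the same experience the owner gains.
; Damage multiplies a base value by a level curve.
; Equip, Unequip and GetDamageLocations are empty; ability grant and removal logic, including destroy on removal, exists but is unwired.
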(event Custom|ExperienceGained
  (params (XPContext :type S%20XP%20Context%20Structure))
  ;[0 0 0] Adds XP to player
  (Default|AwardXP (Variables|Default|GetBPC_XP) (.ExperienceAdded (Utilities|Struct|BreakS_XPContext XPContext))))

(event Custom|Unequip
  ;[0 0 0] Unequips weapon and removes abilities
)

(event Custom|Equip
  ;[0 0 0] Equips weapon and grants accosiated abilities
)

(event EventBeginPlay
  (bind _returnvalue (Components|GetOwner))
  (bind _returnvalue_2 (Actor|GetComponentbyClass _returnvalue "/Game/Blueprints/XP/BPC_XP.BPC_XP_C"))
  (Utilities|IsValid _returnvalue_2
    (:Is%20Valid
      (EventDispatchers|BindEventtoXPChanged _returnvalue_2 (delegate Custom|ExperienceGained)))))

(fn ConstructionScript)

(fn GetWeaponDamage
  (return (* (Math|Curves|GetFloatValue (Variables|Default|GetLevelDamageCurve) (Math|Conversions|ToFloat(Integer) (Variables|/Game/Blueprints/XP/BPC_XP.BPC_XP_C|GetCurrentLevel (Variables|Default|GetBPC_XP)))) (Variables|Default|GetDamageValue))))

(fn GetDamageLocations
  ;[0 0 0] Should return all sets of points that should scan for damage. Skeletal mesh of the weapon determines points
  (return 0))
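; Base status effect that temporarily changes its owner's gameplay tags and attributes, with a periodic hook for child classes such as poison ticks.
; AttemptApplication checks required and preventing tags, then either starts the effect or attempts its removal.
; Starting adds tags, applies curve-scaled attribute changes by Level, and sets periodic and duration timers.
; Expiry removes tags, applies negated attribute changes, clears timers and requests removal from the owner's BPC_StatusEffects.
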(event Custom|AttemptApplication
  ;[0 0 0] Attempting to add a status effect
  ;[0 0 0] Check if we can use status effects
  (bind _applystatuseffect (CallFunction|CheckTagStartConditions))
  (if _applystatuseffect
    (CallFunction|StartStatusEffect)
    (else
      ;[0 0 0] Cannot add status effect, attempt early end
      (Utilities|AttemptRemoveStatusEffects))))

(event Custom|StartStatusEffect
  (bind _statuseffectinfo (Variables|Default|GetStatusEffectInfo))
  (bind (_duration _periodictime) (Utilities|Struct|BreakS_StatusEffects _statuseffectinfo))
  ;[0 0 0] Apply status effect tags
  (CallFunction|AddTags)
  ;[0 0 0] Apply changes to attributs from status effects
  (CallFunction|ApplyAttributeEffects true)
  ;[0 0 0] Set periodic timer (Poison ticks)
  (bind _returnvalue (Utilities|Time|SetTimerbyEvent (delegate Custom|PeriodicEvent) _periodictime true))
  (Variables|Default|SetPeriodicTimerHandle _returnvalue)
  ;[0 0 0] Start the duration timer (lifetime of the effect)
  (bind _returnvalue_2 (Utilities|Time|SetTimerbyEvent (delegate Custom|EndStatusEffect) _duration false 0.001))
  (Variables|Default|SetDurationTimerHandle _returnvalue_2))

(event Custom|PeriodicEvent
  ;[0 0 0] Event to overwrite functionality for perodic effects in child classes
)

(event Custom|EndStatusEffect
  ;[0 0 0] Remove all status effect tags
  (CallFunction|RemoveTags)
  ;[0 0 0] Remove all changes to attributes from status effects
  (CallFunction|ApplyAttributeEffects false)
  ;[0 0 0] Clear all timer handles
  (CallFunction|ClearTimers)
  (Utilities|AttemptRemoveStatusEffects))

(event EventBeginPlay)

(fn ConstructionScript)

(fn ClearTimers
  ;[0 0 0] Clear all timer handles
  (Utilities|Time|ClearandInvalidateTimerbyHandle (Variables|Default|GetPeriodicTimerHandle))
  (Utilities|Time|ClearandInvalidateTimerbyHandle (Variables|Default|GetDurationTimerHandle))
  (return))

(fn CheckTagStartConditions
  ;[0 0 0] Check if we can add a status effect
  (bind _tagcontainer (Default|GetActiveTagContainer (Actor|GetComponentbyClass (Components|GetOwner) "/Game/Blueprints/GamePlayTags/BPC_GameplayTags.BPC_GameplayTags_C")))
  (return (and (GameplayTags|HasAllTags _tagcontainer (Variables|Default|GetRequiredTags)) (not (GameplayTags|HasAnyTags _tagcontainer (Variables|Default|GetPreventingTags))))))

(fn AddTags
  (bind _returnvalue (Components|GetOwner))
  ;[0 0 0] Apply status effect tags
  (for _array_element (Variables|Default|GetAddingTags)
    (Default|AddTag (Actor|GetComponentbyClass _returnvalue "/Game/Blueprints/GamePlayTags/BPC_GameplayTags.BPC_GameplayTags_C") _array_element (Utilities|Struct|MakeS_Origin _returnvalue (Game|GetInstigatorController _returnvalue))))
  (return))

(fn RemoveTags
  (bind _returnvalue (Components|GetOwner))
  ;[0 0 0] Remove all status effect tags
  (for _array_element (Variables|Default|GetAddingTags)
    (Default|RemoveTag (Actor|GetComponentbyClass _returnvalue "/Game/Blueprints/GamePlayTags/BPC_GameplayTags.BPC_GameplayTags_C") _array_element (Utilities|Struct|MakeS_Origin _returnvalue (Game|GetInstigatorController _returnvalue))))
  (return))

(fn ApplyAttributeEffects
  (params (AddEffects :type Boolean))
  (bind _returnvalue (Components|GetOwner))
  (bind _returnvalue_2 (Actor|GetComponentbyClass _returnvalue "/Game/Blueprints/Attributes/BPC_Attributes.BPC_Attributes_C"))
  ;[0 0 0] Add or remove attribute effects from the status effects config
  (if AddEffects
    ;[0 0 0] Add or remove?
    (LocalVariables|SetLocalMultiplier 1.0)
    (else
      (LocalVariables|SetLocalMultiplier -1.0)))
  ;[0 0 0] do we have an attribute component
  (Utilities|IsValid _returnvalue_2
    (:Is%20Valid
      (for _array_element (Variables|Default|GetAttributeEffects)
        ;[0 0 0] Can go through all attributes to change and apply change
        (Default|ChangeAttribute _returnvalue_2 (.AttributeToChange (Utilities|Struct|BreakS_AttributeChange _array_element)) (* (* (.PowerMultiplier (Utilities|Struct|BreakS_AttributeChange _array_element)) (Math|Curves|GetFloatValue (.ScalingCurve (Utilities|Struct|BreakS_AttributeChange _array_element)) (Variables|Default|GetLevel))) (LocalVariables|GetLocalMultiplier)) (.ChangeType (Utilities|Struct|BreakS_AttributeChange _array_element)) (Utilities|Struct|MakeS_Origin (Components|GetOwner) (Game|GetInstigatorController))))
      (return))
    (:Is%20Not%20Valid
      (return))))
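; Room trigger volume that activates the wave spawn points inside it when the player character enters.
; Entry stores the player, tags each overlapped BP_WaveSpawnPoint "Active" and spawns a small Niagara shield effect there, with a delayed destroy.
; After the loop it removes the tag from only the last point and caches overlapping BP_EnemyBase actors as room enemies.
; Player exit clears that list and re-arms the trigger.
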(event OnComponentBeginOverlap(Trigger)
  (params (OverlappedComponent :type Primitive%20Component%20Object%20Reference) (OtherActor :type Actor%20Object%20Reference) (OtherComp :type Primitive%20Component%20Object%20Reference) (OtherBodyIndex :type Integer) (bFromSweep :type Boolean) (SweepResult :type Hit%20Result%20Structure%20%28by%20ref%29))
  (if (not (Variables|Default|GetTriggered))
    (bind _asbp_third_person_character (Utilities|Casting|CastToBP_ThirdPersonCharacter OtherActor))
    (Variables|Default|SetPlayerREF _asbp_third_person_character)
    (Variables|Default|SetTriggered true)
    (for _array_element (Collision|GetOverlappingActors (Variables|Default|GetTrigger) "/Game/Blueprints/AI/Spawner/BP_WaveSpawnPoint.BP_WaveSpawnPoint_C" :!class /Script/Engine.PrimitiveComponent)
      (Utilities|Array|Add (Variables|/Script/Engine.Actor|GetTags _array_element) "Active")
      (bind _returnvalue (Niagara|SpawnSystematLocation "/Game/VFX/WizardSpellsPack/Effects/NS_Shield_buff.NS_Shield_buff" (Transformation|GetActorLocation _array_element) "0, 0, 0" "0.100000,0.100000,0.100000"))
      (Utilities|FlowControl|Delay 0.5)
      (Components|DestroyComponent _returnvalue))
    (Utilities|Array|RemoveItem (Variables|/Script/Engine.Actor|GetTags _array_element) "Active")
    (Variables|Default|SetCurrentRoomEnemies (Collision|GetOverlappingActors "/Game/Blueprints/AI/Blueprints/Enemies/BP_EnemyBase.BP_EnemyBase_C" :!class /Script/Engine.Actor))))

(event OnComponentEndOverlap(Trigger)
  (params (OverlappedComponent :type Primitive%20Component%20Object%20Reference) (OtherActor :type Actor%20Object%20Reference) (OtherComp :type Primitive%20Component%20Object%20Reference) (OtherBodyIndex :type Integer))
  (Utilities|Casting|CastToBP_ThirdPersonCharacter OtherActor)
  (Utilities|Array|Clear (Variables|Default|GetCurrentRoomEnemies))
  (Variables|Default|SetTriggered false))

(event EventBeginPlay)

(event Collision|EventActorBeginOverlap
  (params (OtherActor :type Actor%20Object%20Reference)))

(event EventTick
  (params (DeltaSeconds :type Float%20%28single-precision%29)))

(fn ConstructionScript)
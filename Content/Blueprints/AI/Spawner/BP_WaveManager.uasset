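; Wave manager that spawns enemies when the room trigger fires and unlocks exit doors once they are dead.
; It sorts "Active"-tagged spawn points by enemy type, then reads the data table row named after the wave number.
; Each enemy spawns at the last point in its type's list.
; A one-second polling loop detects the clear, advances the wave, briefly shows a widget and binds the trigger's end event to restart.
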(event Custom|SpawnerEnded
  (CallFunction|SpawnerBegin))

(event Custom|BeginWave
  (bind _returnvalue (Utilities|GetDataTableRow (Variables|Default|GetEnemyDataTable) (Utilities|String|StringToName (Utilities|String|ToString(Integer) (Variables|Default|GetWaveNumber))))
    (:then
      (for _array_element (Utilities|Struct|BreakS_WaveInfo _returnvalue)
        (CallFunction|SpawnEnemies _array_element))
      (CallFunction|StartCheckingifEnemiesAreDead))
    (:RowNotFound
      (Development|PrintString "No Row Found!"))))

(event Custom|StartCheckingIfEnemiesAreDead
  (bind _isdead (CallFunction|CheckifAllEnemiesAreDead :!label _label))
  (if _isdead
    (Math|Integer|IncrementInt (Variables|Default|GetWaveNumber)
      (:%20%20
        (for _array_element (Variables|Default|GetExitDoors)
          (Variables|/Game/MedievalDungeon/Blueprints/BP_Dungeon_Doorway.BP_Dungeon_Doorway_C|SetLocked _array_element false))
        (bind _returnvalue (UserInterface|CreateWidget "/Game/Widgets/Screens/WB_DoorsUnlockedScreen.WB_DoorsUnlockedScreen_C" (Game|GetPlayerController 0)))
        (UserInterface|Viewport|AddtoViewport _returnvalue 0)
        (Utilities|FlowControl|Delay 1.0)
        (Widget|RemovefromParent _returnvalue)
        (EventDispatchers|AssignEndSpawner (Variables|Default|GetRoomTrigger) (delegate Custom|SpawnerEnded))))
    (else
      (Utilities|FlowControl|Delay 1.0)
      (goto _label))))

(event Custom|SpawnerBegin
  (bind _outactors (Actor|GetAllActorsOfClass "/Game/Blueprints/AI/Spawner/BP_WaveSpawnPoint.BP_WaveSpawnPoint_C"))
  (bind _output_get (Variables|Default|SetEnemySpawnPoints _outactors))
  (for _array_element _output_get
    (if (Actor|ActorHasTag _array_element "Active")
      (Utilities|IsValid _array_element
        (:Is%20Valid
          (switch Utilities|FlowControl|Switch|SwitchonE_EnemyTypes (Variables|/Game/Blueprints/AI/Spawner/BP_WaveSpawnPoint.BP_WaveSpawnPoint_C|GetSpawnerType _array_element)
            (:NewEnumerator0
              (Utilities|Array|Add (Variables|Default|GetMeleeSpawnPoints) _array_element))
            (:NewEnumerator1
              (Utilities|Array|Add (Variables|Default|GetRangedSpawnPoints) _array_element))
            (:NewEnumerator2
              (Utilities|Array|Add (Variables|Default|GetMageSpawnPoints) _array_element)))))))
  (Utilities|FlowControl|Delay 5.0)
  (CallFunction|BeginWave))

(event EventBeginPlay
  (bind _returnvalue (Actor|GetActorOfClass "/Game/Blueprints/AI/Spawner/BP_RoomTrigger.BP_RoomTrigger_C"))
  (bind _output_get (Variables|Default|SetRoomTrigger _returnvalue))
  (EventDispatchers|AssignBeginSpawner _output_get (delegate Custom|SpawnerBegin)))

(fn ConstructionScript)

(fn SpawnEnemies
  (params (S_EnemyInfo :type S%20Enemy%20Info%20Structure%20%28by%20ref%29))
  (LocalVariables|SetEnemyInfoREF S_EnemyInfo)
  (LocalVariables|SetCurrentSpawnPoints (Utilities|Select :Index (.EnemyType (Utilities|Struct|BreakS_EnemyInfo S_EnemyInfo)) :NewEnumerator0 (Variables|Default|GetMeleeSpawnPoints) :NewEnumerator1 (Variables|Default|GetRangedSpawnPoints) :NewEnumerator2 (Variables|Default|GetMageSpawnPoints)))
  (for _index (range 1 (.enemynumber (LocalVariables|GetEnemyInfoREF)))
    (bind _returnvalue (Game|SpawnActorfromClass (.enemyclass (LocalVariables|GetEnemyInfoREF)) (Transformation|GetWorldTransform (Variables|/Game/Blueprints/AI/Spawner/BP_WaveSpawnPoint.BP_WaveSpawnPoint_C|GetBillboard (Utilities|Array|Get(acopy) (LocalVariables|GetCurrentSpawnPoints) (Utilities|Array|LastIndex (LocalVariables|GetCurrentSpawnPoints))))) "AdjustIfPossibleButAlwaysSpawn" "MultiplyWithRoot" 0 0))
    (Utilities|Array|Add (Variables|Default|GetCurrentEnemies) _returnvalue)))

(fn CheckifAllEnemiesAreDead
  (LocalVariables|SetAreDead true)
  (for _array_element (Variables|Default|GetCurrentEnemies)
    (Utilities|IsValid _array_element
      (:Is%20Valid
        (LocalVariables|SetAreDead false))))
  (return (LocalVariables|GetAreDead)))
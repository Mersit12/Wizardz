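; AI character Blueprint that uses perception to decide which target it follows, with a short memory after losing it.
; On each perception update, every successfully sensed stimulus writes its actor to the PlayerTarget blackboard key and cancels the forget timer.
; A failed stimulus starts a MemoryDuration timer, which clears PlayerTarget when it expires.
; Any perceived actor can become PlayerTarget, as no player check is made.
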(event OnPerceptionUpdated(AIPerception)
  (params (UpdatedActors :type Array%20of%20Actor%20Object%20References))
  (bind _returnvalue (AI|GetBlackboard 0))
  (for _array_element UpdatedActors
    (bind _info (Class|AIPerceptionComponent|GetActorsPerception (Variables|Default|GetAIPerception) _array_element))
    (for _array_element_2 (.LastSensedStimuli (Utilities|Struct|BreakActorPerceptionBlueprintInfo _info))
      (if (.bSuccessfullySensed (Utilities|Struct|BreakAIStimulus _array_element_2))
        ;[0 0 0] AI has seen the player, store value in blackboard
        (Utilities|IsValid _returnvalue
          (:Is%20Valid
            (AI|Components|Blackboard|SetValueasObject _returnvalue (Utilities|Name|MakeLiteralName "PlayerTarget") (.Target (Utilities|Struct|BreakActorPerceptionBlueprintInfo _info)))
            (Utilities|Time|ClearandInvalidateTimerbyHandle (Variables|Default|GetRememberPlayerTimerREF))))
        (else
          ;[0 0 0] AI Lost line of sight, start timer to reflect how long it remains following the pplayer
          (bind _returnvalue_2 (Utilities|Time|SetTimerbyEvent (delegate Custom|StopFollowingPlayer) (Variables|Default|GetMemoryDuration)))
          (Variables|Default|SetRememberPlayerTimerREF _returnvalue_2))))))

(event Custom|StopFollowingPlayer
  (bind _returnvalue (AI|GetBlackboard 0))
  ;[0 0 0] Player should no longer be followed as AI has lost sight for too long
  (Utilities|IsValid _returnvalue
    (:Is%20Valid
      (AI|Components|Blackboard|SetValueasObject _returnvalue (Utilities|Name|MakeLiteralName "PlayerTarget") 0))))

(event EventBeginPlay
  (|CallParentFunction) ; This node is disabled and will not be called.\nDrag off pins to build functionality.
)

(event Collision|EventActorBeginOverlap
  (params (OtherActor :type Actor%20Object%20Reference)))

(event EventTick
  (params (DeltaSeconds :type Float%20%28single-precision%29)))

(fn ConstructionScript
  (|CallParentFunction))
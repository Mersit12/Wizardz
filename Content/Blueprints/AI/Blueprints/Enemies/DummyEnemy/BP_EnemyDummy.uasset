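; Training-dummy enemy Blueprint that complains in on-screen dialogue whenever it takes damage.
; On BeginPlay it runs the parent logic and flags its AI controller as a dummy enemy.
; Each hit runs parent damage handling, then replaces any dialogue box with the next indexed line.
; Delays then dismiss the widget and reset the HUD, after which the line index wraps.
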(event EventBeginPlay
  (|CallParentFunction)
  (Variables|/Game/Blueprints/AI/Blueprints/Enemies/BP_EnemyAIController.BP_EnemyAIController_C|SetDummyEnemy (Variables|Default|GetAiControllerREF) true))

(event Collision|EventActorBeginOverlap
  (params (OtherActor :type Actor%20Object%20Reference)))

(event EventTick
  (params (DeltaSeconds :type Float%20%28single-precision%29)))

(event Game|Damage|EventAnyDamage
  (params (Damage :type Float%20%28single-precision%29) (DamageType :type Damage%20Type%20Object%20Reference) (InstigatedBy :type Controller%20Object%20Reference) (DamageCauser :type Actor%20Object%20Reference))
  (|CallParentFunction Damage DamageType InstigatedBy DamageCauser)
  (Math|Integer|IncrementInt (Variables|Default|GetDialogueIndex)
    (:%20%20
      (Utilities|IsValid (Variables|Default|GetDialogueBoxREF)
        (:Is%20Valid
          (Widget|RemovefromParent (Variables|Default|GetDialogueBoxREF)))
        (:Is%20Not%20Valid
          _))
      (bind _returnvalue (UserInterface|CreateWidget "/Game/Widgets/Dialogue/W_DialogueBox.W_DialogueBox_C"))
      (bind _output_get (Variables|Default|SetDialogueBoxREF _returnvalue))
      (Variables|/Game/Widgets/Dialogue/W_DialogueBox.W_DialogueBox_C|SetDialogueText _output_get (Utilities|Select :Index (Variables|Default|GetDialogueIndex) :Option%200 "Ow!" :Option%201 "That Hurt!" :Option%202 "Stop!!!" :Option%203 "What kind of madness is this?!" :Option%204 "Control yourself, sir!" :Option%205 "Please Stop!" :Option%206 "Are you getting bored yet?" :Option%207 "No... ok this is getting ridiculous!"))
      (UserInterface|Viewport|AddtoViewport _output_get 0)
      (Utilities|FlowControl|Delay 3.0)
      (Default|RemoveDialogueBox (Variables|Default|GetDialogueBoxREF))
      (Utilities|FlowControl|Delay 0.2)
      (Default|ResetHUD (Variables|Default|GetDialogueBoxREF))
      (Widget|RemovefromParent (Variables|Default|GetDialogueBoxREF))
      (if (>= (Variables|Default|GetDialogueIndex) 8)
        (Variables|Default|SetDialogueIndex 0)))))

(fn ConstructionScript
  (|CallParentFunction))
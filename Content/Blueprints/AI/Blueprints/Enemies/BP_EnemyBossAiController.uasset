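; AI controller for the enemy boss, extending the parent enemy controller's attack and sight behavior.
; On entering the attack state against the player, it adds the boss's health bar to the player HUD's top vertical box, guarded by a DoOnce that resets if the target isn't the player.
; HandleLostSight is overridden empty so the boss never loses track of the player.
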(event EventBeginPlay)

(event EventTick
  (params (DeltaSeconds :type Float%20%28single-precision%29)))

(fn ConstructionScript
  (|CallParentFunction))

(fn SetStateasAttacking
  (params (AttackTarget :type Actor%20Object%20Reference))
  (|CallParentFunction AttackTarget)
  (Utilities|FlowControl|DoOnce false :!label _label
    (:Completed
      (bind _asbp_third_person_character (Utilities|Casting|CastToBP_ThirdPersonCharacter AttackTarget)
        (:then
          (bind _asbp_enemy_boss (Utilities|Casting|CastToBP_EnemyBoss (Pawn|GetControlledPawn)))
          (Class|VerticalBox|AddChildtoVerticalBox (Variables|/Game/Widgets/HUD/W_HUD.W_HUD_C|GetTopVerticalBox (Variables|/Game/PlayerCharacter/ThirdPerson/Blueprints/BP_ThirdPersonCharacter.BP_ThirdPersonCharacter_C|GetPlayerHUDREF _asbp_third_person_character)) (Variables|/Game/Blueprints/AI/Blueprints/Enemies/BossEnemy/BP_EnemyBoss.BP_EnemyBoss_C|GetBossHealthBarREF _asbp_enemy_boss)))
        (:CastFailed
          (goto _label Reset))))))

(fn HandleLostSight
  (params (Actor :type Actor%20Object%20Reference))
  ;[0 0 0] Override to prevent boss losing sight of player
)
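; BP_SpeedBoost is an environmental trigger that gives a temporary speed boost to any BP_MageClass that touches it.
; Box overlap raises the mage's MaxWalkSpeed, then a short Delay resets it to a hardcoded value rather than the previous one.
; It also offsets the mage's max jump height into a MaxJumpHeight variable and later reverts it, without writing it back to CharacterMovement.
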(event OnComponentBeginOverlap(Box)
  (params (OverlappedComponent :type Primitive%20Component%20Object%20Reference) (OtherActor :type Actor%20Object%20Reference) (OtherComp :type Primitive%20Component%20Object%20Reference) (OtherBodyIndex :type Integer) (bFromSweep :type Boolean) (SweepResult :type Hit%20Result%20Structure%20%28by%20ref%29))
  (bind _asbp_mage_class (Utilities|Casting|CastToBP_MageClass OtherActor))
  (Variables|/Script/Engine.CharacterMovementComponent|SetMaxWalkSpeed (Variables|/Script/Engine.Character|GetCharacterMovement _asbp_mage_class) 1e+03)
  (Variables|Default|SetMaxJumpHeight (+ (Class|CharacterMovementComponent|GetMaxJumpHeight (Variables|/Script/Engine.Character|GetCharacterMovement _asbp_mage_class)) 5e+01))
  (Utilities|FlowControl|Delay 1.5)
  (Variables|/Script/Engine.CharacterMovementComponent|SetMaxWalkSpeed (Variables|/Script/Engine.Character|GetCharacterMovement _asbp_mage_class) 6e+02)
  (Variables|Default|SetMaxJumpHeight (- (Variables|Default|GetMaxJumpHeight) 5e+01)))

(event EventBeginPlay)

(event Collision|EventActorBeginOverlap
  (params (OtherActor :type Actor%20Object%20Reference)))

(event EventTick
  (params (DeltaSeconds :type Float%20%28single-precision%29)))

(fn ConstructionScript)
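; Actor component that manages the abilities available to its owning pawn.
; It spawns each ability class as an actor owned and instigated by the pawn, stores it in an array, and triggers its use by index.
; Adding or removing by class broadcasts the updated list, and removal does not destroy the spawned actor.
; ResetAbilities only copies the first entry into index 1, without clearing the array or broadcasting.
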(event EventBeginPlay
  ;[0 0 0] Saving pawn reference for later use
  (bind _aspawn (Utilities|Casting|CastToPawn (Components|GetOwner)))
  (Variables|Default|SetOwnerPawnRef _aspawn))

(fn AddAbilitybyClass
  (params (AbilityClass :type BP%20Ability%20Class%20Reference))
  (bind _ownerpawnref (Variables|Default|GetOwnerPawnRef))
  ;[0 0 0] Create and add ability from input
  (bind _returnvalue (Game|SpawnActorfromClass AbilityClass (Math|Transform|MakeTransform "0, 0, 0" "0, 0, 0" "1.000000,1.000000,1.000000") "Undefined" "SelectDefaultAtRuntime" _ownerpawnref _ownerpawnref))
  (Utilities|Array|Add (Variables|Default|GetAvailableAblilities) _returnvalue)
  ;[0 0 0] Inform that abilities were updated
  (Default|CallAbilitiesAvailableChanged (Variables|Default|GetAvailableAblilities))
  (return))

(fn UseAbility
  (params (AbilityIndex :type Integer))
  (bind _availableablilities (Variables|Default|GetAvailableAblilities))
  (bind _output (Utilities|Array|Get(acopy) _availableablilities AbilityIndex))
  (Utilities|IsValid _output
    (:Is%20Valid
      (Default|AttemptUseAbility _output)
      (return))))

(fn InitializeAbilities
  (params (KnownAbilities :type Array%20of%20BP%20Ability%20Class%20References))
  ;[0 0 0] Funciton to initialize abilities from input array
  (for _array_element KnownAbilities
    (CallFunction|AddAbilitybyClass _array_element))
  (return))

(fn RemoveAbilitybyClass
  (params (AbilityClass :type BP%20Ability%20Class%20Reference))
  (bind _availableablilities (Variables|Default|GetAvailableAblilities))
  (for _array_element _availableablilities
    (if (== (Utilities|GetClass _array_element) AbilityClass)
      (Utilities|Array|RemoveItem _availableablilities _array_element)))
  (Default|CallAbilitiesAvailableChanged (Variables|Default|GetAvailableAblilities))
  (return))

(fn ResetAbilities
  (bind _availableablilities (Variables|Default|GetAvailableAblilities))
  (Utilities|Array|SetArrayElem _availableablilities 1 (Utilities|Array|Get(acopy) _availableablilities))
  (return))
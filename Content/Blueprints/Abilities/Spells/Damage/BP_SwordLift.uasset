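; BP_SwordLift is a damage spell ability that fires a stationary, upward sword projectile with an explosion radius.
; On the animation apex event, it sets the sword-up projectile class and air-attack Niagara effect on the owner's BPC_Combat component, then calls FireProjectile.
; Damage comes from a level curve sampled at the current ability level, scaled by a power multiplier.
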(event EventBeginPlay
  (|CallParentFunction) ; This node is disabled and will not be called.\nDrag off pins to build functionality.
)

(event EventAnimationApexEvent
  (bind _returnvalue (Components|GetOwner))
  (bind _returnvalue_2 (Actor|GetComponentbyClass _returnvalue "/Game/Blueprints/Combat/BPC_Combat.BPC_Combat_C"))
  (Variables|/Game/Blueprints/Combat/BPC_Combat.BPC_Combat_C|SetProjectileType _returnvalue_2 "/Game/Blueprints/Abilities/Projectiles/BP_ProjectileSwordUp.BP_ProjectileSwordUp_C")
  (Variables|/Game/Blueprints/Combat/BPC_Combat.BPC_Combat_C|SetSpellParticle _returnvalue_2 "/Game/WizardSpellsPack/Effects/NS_Sword_air_attack.NS_Sword_air_attack")
  (Default|FireProjectile _returnvalue_2 (Utilities|Struct|MakeS_ProjectileStats (* (Math|Curves|GetFloatValue (Variables|Default|GetLevelCurve) (Variables|Default|GetCurrentAbilityLevel)) (Variables|Default|GetPowerMultiplier)) (Variables|Default|GetSpeed) (Variables|Default|GetExplosion%20Radius) true true)))

(fn ConstructionScript
  (|CallParentFunction))
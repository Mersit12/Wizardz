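; BP_ElecOrb is a damage spell ability that fires an electric orb projectile.
; On the animation apex event it starts its cooldown count, then sets the projectile class and muzzle Niagara effect on the owner's BPC_Combat component.
; That component fires the projectile using stats from CreateProjectileStats.
; A lightning sound plays at player 0's location rather than the owner's.
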(event EventBeginPlay
  (|CallParentFunction) ; This node is disabled and will not be called.\nDrag off pins to build functionality.
)

(event EventAnimationApexEvent
  (bind _returnvalue (Components|GetOwner))
  (bind _returnvalue_2 (Actor|GetComponentbyClass _returnvalue "/Game/Blueprints/Combat/BPC_Combat.BPC_Combat_C"))
  (CallFunction|CooldownCount)
  (Variables|/Game/Blueprints/Combat/BPC_Combat.BPC_Combat_C|SetProjectileType _returnvalue_2 "/Game/Blueprints/Abilities/Projectiles/BP_ProjectileElecOrb.BP_ProjectileElecOrb_C")
  (Variables|/Game/Blueprints/Combat/BPC_Combat.BPC_Combat_C|SetSpellParticle _returnvalue_2 "/Game/VFX/WizardSpellsPack/sA_Megapack_v1/sA_Projectilevfx/Vfx/Fx/Niagara_Systems/NS_Muzzle_4.NS_Muzzle_4")
  (Default|FireProjectile _returnvalue_2 (CallFunction|CreateProjectileStats))
  (Audio|PlaySoundatLocation "/Game/VFX/WizardSpellsPack/Audio/S_Lightning_3.S_Lightning_3" (Transformation|GetActorLocation (Game|GetPlayerCharacter 0)) "0, 0, 0" 1.0 1.0 0.0 0 0 0 0))

(fn ConstructionScript
  (|CallParentFunction))
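; BP_RedBeam is a damage spell ability that fires a beam at the apex of its animation.
; The apex event spawns a BP_BeamSpawn at the owner's spell spawn transform, passing high-damage, zero-speed projectile stats, the owner and the instigating pawn.
; It also spawns an energy Niagara effect there, nudged along world X rather than the caster's facing.
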(event EventBeginPlay
  (|CallParentFunction) ; This node is disabled and will not be called.\nDrag off pins to build functionality.
)

(event EventAnimationApexEvent
  (bind _returnvalue (Components|GetOwner))
  (bind _spellspawntransform (Class|BPIGetSpellSpawn|GetSpellSpawnLocation(Message) _returnvalue))
  (Game|SpawnActorfromClass "/Game/Blueprints/Abilities/Projectiles/BP_BeamSpawn.BP_BeamSpawn_C" _spellspawntransform "Undefined" "MultiplyWithRoot" _returnvalue (Utilities|Struct|MakeS_ProjectileStats 1e+02 0.0 0.0 false) 0 (Variables|Default|GetPawnREF))
  (bind _spellspawntransform_2 (Class|BPIGetSpellSpawn|GetSpellSpawnLocation(Message) (Components|GetOwner)))
  (Niagara|SpawnSystematLocation "/Game/WizardSpellsPack/sA_Megapack_v1/sA_Rayvfx/Fx/NiagaraSystems/NS_Energy_5.NS_Energy_5" (+ (.location _spellspawntransform_2) "50.000000,0.000000,0.000000") (.rotation _spellspawntransform_2)))

(fn ConstructionScript
  (|CallParentFunction))
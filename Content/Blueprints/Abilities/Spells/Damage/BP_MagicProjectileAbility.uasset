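; Magic projectile damage spell ability that supplies projectile stats scaled to the ability's current level.
; CreateProjectileStats returns damage from a level curve times a power multiplier, along with speed and explosion radius.
; At the animation apex it starts the cooldown count, fetches the owner's combat component and builds a similar stats struct with cooldown, but the graph shows no spawn or further use of either.
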(event EventAnimationApexEvent
  (CallFunction|CooldownCount)
  (Variables|Default|SetBPC_Combat_0 (Actor|GetComponentbyClass (Components|GetOwner) "/Game/Blueprints/Combat/BPC_Combat.BPC_Combat_C"))
  (Variables|Default|SetS%20Projectile%20Stats (Utilities|Struct|MakeS_ProjectileStats (* (Math|Curves|GetFloatValue (Variables|Default|GetLevelCurve) (Variables|Default|GetCurrentAbilityLevel)) (Variables|Default|GetPowerMultiplier)) 3e+03 (Variables|Default|GetExplosion%20Radius) true (Variables|Default|GetCooldown))))

(fn ConstructionScript
  (|CallParentFunction))

(fn CreateProjectileStats
  (return (Utilities|Struct|MakeS_ProjectileStats (* (Math|Curves|GetFloatValue (Variables|Default|GetLevelCurve) (Variables|Default|GetCurrentAbilityLevel)) (Variables|Default|GetPowerMultiplier)) (Variables|Default|GetSpeed) (Variables|Default|GetExplosion%20Radius) true)))
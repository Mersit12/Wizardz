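; Imbue Flames spell that temporarily boosts the player's equipped weapon damage and shows a flame trail.
; At the animation apex event, it adds AddedDamage to the weapon's damage and attaches a Niagara flame system to the character's right hand.
; After ActiveTime, it destroys the effect and sets damage to a hard-coded value rather than restoring the previous one.
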(event EventBeginPlay
  (|CallParentFunction) ; This node is disabled and will not be called.\nDrag off pins to build functionality.
)

(event Collision|EventActorBeginOverlap
  (params (OtherActor :type Actor%20Object%20Reference)))

(event EventTick
  (params (DeltaSeconds :type Float%20%28single-precision%29)))

(event EventAnimationApexEvent
  (bind _asbp_third_person_character (Utilities|Casting|CastToBP_ThirdPersonCharacter (Game|GetPlayerCharacter 0)))
  (Variables|/Game/Blueprints/Weapons/BP_Weapon.BP_Weapon_C|SetDamageValue (Variables|/Game/Blueprints/Combat/BPC_Combat.BPC_Combat_C|GetEquippedWeapon (Variables|/Game/PlayerCharacter/ThirdPerson/Blueprints/BP_ThirdPersonCharacter.BP_ThirdPersonCharacter_C|GetBPC_Combat _asbp_third_person_character)) (+ (Default|GetWeaponDamage (Variables|/Game/Blueprints/Combat/BPC_Combat.BPC_Combat_C|GetEquippedWeapon (Variables|/Game/PlayerCharacter/ThirdPerson/Blueprints/BP_ThirdPersonCharacter.BP_ThirdPersonCharacter_C|GetBPC_Combat _asbp_third_person_character))) (Variables|Default|GetAddedDamage)))
  (bind _returnvalue (Niagara|SpawnSystemAttached "/Game/VFX/WizardSpellsPack/sA_Megapack_v1/sA_StylizedAttacksPack/FX/NiagaraSystems/NS_Flame_Trail.NS_Flame_Trail" (Variables|/Script/Engine.Character|GetMesh _asbp_third_person_character) "Hand_R" "0, 0, 0" "0, 0, 0" "SnapToTarget" false))
  (Utilities|FlowControl|Delay (Variables|Default|GetActiveTime))
  (Variables|/Game/Blueprints/Weapons/BP_Weapon.BP_Weapon_C|SetDamageValue (Variables|/Game/Blueprints/Combat/BPC_Combat.BPC_Combat_C|GetEquippedWeapon (Variables|/Game/PlayerCharacter/ThirdPerson/Blueprints/BP_ThirdPersonCharacter.BP_ThirdPersonCharacter_C|GetBPC_Combat _asbp_third_person_character)) 8e+01)
  (Components|DestroyComponent _returnvalue))

(fn ConstructionScript
  (|CallParentFunction))
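; BP_TelePush is a non-damage spell that shoves an enemy along the owner's forward direction.
; On the animation apex event it runs CooldownCount, then MoveHitActor line traces to the lock-on target, or straight ahead when nothing is locked.
; A hit BP_EnemyBase is launched at a fixed speed with LaunchCharacter.
; Both traces leave persistent debug drawing on.
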(event EventBeginPlay
  (|CallParentFunction) ; This node is disabled and will not be called.\nDrag off pins to build functionality.
)

(event EventAnimationApexEvent
  (CallFunction|CooldownCount)
  (CallFunction|MoveHitActor))

(fn ConstructionScript
  (|CallParentFunction))

(fn MoveHitActor
  (bind _returnvalue (Components|GetOwner))
  (bind _returnvalue_2 (Components|GetOwner))
  (bind _returnvalue_3 (Components|GetOwner))
  (bind _returnvalue_4 (Actor|GetComponentbyClass _returnvalue_3 "/Script/LockOnTarget.LockOnTargetComponent"))
  (bind _returnvalue_5 (Transformation|GetActorLocation _returnvalue_2))
  (if (Class|LockonTargetComponent|IsTargetLocked _returnvalue_4)
    (bind _outhit (Collision|LineTraceByChannel (Transformation|GetActorLocation _returnvalue) (Transformation|GetActorLocation (Class|LockonTargetComponent|GetTargetActor _returnvalue_4)) "TraceTypeQuery3" false (Utilities|Array|MakeArray _returnvalue) "Persistent"))
    (bind _asbp_enemy_base (Utilities|Casting|CastToBP_EnemyBase (.HitActor (Collision|BreakHitResult _outhit))))
    (Character|LaunchCharacter _asbp_enemy_base (* (Math|Vector|GetForwardVector (Transformation|GetActorRotation (Components|GetOwner))) 1.5e+03) false false)
    (else
      (bind _outhit_2 (Collision|LineTraceByChannel _returnvalue_5 (+ _returnvalue_5 (* (Transformation|GetActorForwardVector _returnvalue_2) 1e+04)) "TraceTypeQuery3" false (Utilities|Array|MakeArray (Components|GetOwner)) "Persistent"))
      (bind _asbp_enemy_base_2 (Utilities|Casting|CastToBP_EnemyBase (.HitActor (Collision|BreakHitResult _outhit_2))))
      (Character|LaunchCharacter _asbp_enemy_base_2 (* (Math|Vector|GetForwardVector (Transformation|GetActorRotation (Components|GetOwner))) 1.5e+03) false false))))
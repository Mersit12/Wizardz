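; BP_GroundStun is a non-damage spell that sinks an enemy into the ground and freezes it.
; At the animation apex it starts its cooldown and line-traces from the owner to the locked-on target, or straight ahead without a lock.
; A hit enemy stops moving and its AI enters the frozen state while a timeline lerps it downward.
; When the timeline finishes, the AI resumes attacking its target, with no move back up.
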(event EventBeginPlay
  (|CallParentFunction) ; This node is disabled and will not be called.\nDrag off pins to build functionality.
)

(event EventAnimationApexEvent
  (CallFunction|CooldownCount)
  (bind _enemy (CallFunction|MoveHitActor))
  (bind _asbp_enemy_aicontroller (Utilities|Casting|CastToBP_EnemyAIController (AI|GetAIController _enemy)))
  (Variables|Default|SetAiControllerREF _asbp_enemy_aicontroller)
  (Components|Movement|StopMovementImmediately (Variables|/Script/Engine.Character|GetCharacterMovement _enemy))
  (Default|SetStateasFrozen _asbp_enemy_aicontroller)
  (bind _moveintoground (Timeline|MoveEnemy PlayFromStart)
    (:Update
      (Transformation|SetActorLocation _enemy (Math|Vector|Lerp(Vector) (Transformation|GetActorLocation _enemy) (Math|Vector|MakeVector (.x (Transformation|GetActorLocation _enemy)) (.y (Transformation|GetActorLocation _enemy)) (- (.z (Transformation|GetActorLocation _enemy)) 75.0)) _moveintoground) false true))
    (:Finished
      (Default|SetStateasAttacking (Variables|Default|GetAiControllerREF) (Variables|/Game/Blueprints/AI/Blueprints/Enemies/BP_EnemyAIController.BP_EnemyAIController_C|GetAttackTarget _asbp_enemy_aicontroller)))))

(fn ConstructionScript
  (|CallParentFunction))

(fn MoveHitActor
  (bind _returnvalue (Components|GetOwner))
  (bind _returnvalue_2 (Components|GetOwner))
  (bind _returnvalue_3 (Components|GetOwner))
  (bind _returnvalue_4 (Actor|GetComponentbyClass _returnvalue_3 "/Script/LockOnTarget.LockOnTargetComponent"))
  (bind _returnvalue_5 (Transformation|GetActorLocation _returnvalue_2))
  (if (Class|LockonTargetComponent|IsTargetLocked _returnvalue_4)
    (bind _outhit (Collision|LineTraceByChannel (Transformation|GetActorLocation _returnvalue) (Transformation|GetActorLocation (Class|LockonTargetComponent|GetTargetActor _returnvalue_4)) "TraceTypeQuery3" false (Utilities|Array|MakeArray _returnvalue) "None"))
    (bind _asbp_enemy_base (Utilities|Casting|CastToBP_EnemyBase (.HitActor (Collision|BreakHitResult _outhit))))
    (return _asbp_enemy_base)
    (else
      (bind _outhit_2 (Collision|LineTraceByChannel _returnvalue_5 (+ _returnvalue_5 (* (Transformation|GetActorForwardVector _returnvalue_2) 1e+04)) "TraceTypeQuery3" false (Utilities|Array|MakeArray (Components|GetOwner)) "None"))
      (bind _asbp_enemy_base_2 (Utilities|Casting|CastToBP_EnemyBase (.HitActor (Collision|BreakHitResult _outhit_2))))
      (return _asbp_enemy_base_2))))
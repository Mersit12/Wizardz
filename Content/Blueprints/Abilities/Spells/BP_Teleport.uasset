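; Teleport spell Blueprint that fakes a blink as a brief, invisible high-speed flight of the player character.
; At the animation apex, it switches movement to very fast flying, hides the mesh, ignores Pawn collision and plays cast VFX and sound.
; After a short delay, TeleportEnd stops movement, restores walking, visibility and collision, then plays an end montage.
; The OnTeleportEnd dispatcher fires when that montage completes or is interrupted.
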(event Custom|TeleportEnd
  (bind _characterref (Variables|Default|GetCharacterREF))
  (bind _mesh (Variables|/Script/Engine.Character|GetMesh _characterref))
  (bind _charactermovement (Variables|/Script/Engine.Character|GetCharacterMovement _characterref))
  (Components|Movement|StopMovementImmediately _charactermovement)
  (Pawn|Components|CharacterMovement|SetMovementMode _charactermovement "MOVE_Walking" 0)
  (Variables|/Script/Engine.CharacterMovementComponent|SetMaxAcceleration _charactermovement 1e+03)
  (Rendering|SetVisibility _mesh true true)
  (Collision|SetCollisionResponsetoChannel (Variables|/Script/Engine.Character|GetCapsuleComponent (Variables|Default|GetCharacterREF)) "ECC_Pawn" "ECR_Block")
  (Audio|PlaySoundatLocation "/Game/WizardSpellsPack/Audio/Cues/S_Magic_hit_1_Cue.S_Magic_hit_1_Cue" (Transformation|GetActorLocation (Variables|Default|GetCharacterREF)) "0, 0, 0" 1.0 1.0 0.0 0 0 0 0)
  (Animation|Montage|PlayMontage _mesh "/Game/PlayerCharacter/Animations/UE5_WZ_Teleport_01_End_Seq_Montage.UE5_WZ_Teleport_01_End_Seq_Montage"
    (:OnCompleted
      _)
    (:OnInterrupted
      _))
  (Default|CallOnTeleportEnd))

(event EventBeginPlay
  (|CallParentFunction))

(event Collision|EventActorBeginOverlap
  (params (OtherActor :type Actor%20Object%20Reference)))

(event EventTick
  (params (DeltaSeconds :type Float%20%28single-precision%29)))

(event EventAnimationApexEvent
  (bind _asbp_third_person_character (Utilities|Casting|CastToBP_ThirdPersonCharacter (Game|GetPlayerCharacter 0)))
  (bind _output_get (Variables|Default|SetCharacterREF _asbp_third_person_character))
  (Pawn|Components|CharacterMovement|SetMovementMode (Variables|/Script/Engine.Character|GetCharacterMovement _output_get) "MOVE_Flying" 0)
  (Variables|/Script/Engine.CharacterMovementComponent|SetMaxFlySpeed (Variables|/Script/Engine.Character|GetCharacterMovement _output_get) 7e+03)
  (Variables|/Script/Engine.CharacterMovementComponent|SetMaxAcceleration (Variables|/Script/Engine.Character|GetCharacterMovement _output_get) 99999.0)
  (Rendering|SetVisibility (Variables|/Script/Engine.Character|GetMesh _output_get) false true)
  (Collision|SetCollisionResponsetoChannel (Variables|/Script/Engine.Character|GetCapsuleComponent (Variables|Default|GetCharacterREF)) "ECC_Pawn" "ECR_Ignore")
  (Niagara|SpawnSystemAttached "/Game/WizardSpellsPack/Effects/NS_Time_cast.NS_Time_cast" (Variables|/Script/Engine.Character|GetMesh (Variables|Default|GetCharacterREF)) "Spine_01" "0, 0, 0" "90.000000,0.000000,0.000000" "SnapToTarget" false)
  (Audio|PlaySoundatLocation "/Game/WizardSpellsPack/Audio/S_Magic_hit_1.S_Magic_hit_1" (Transformation|GetActorLocation (Variables|Default|GetCharacterREF)) "0, 0, 0" 1.0 1.0 0.0 0 0 0 0)
  (Utilities|FlowControl|Delay 0.3)
  (CallFunction|TeleportEnd))

(fn ConstructionScript
  (|CallParentFunction))
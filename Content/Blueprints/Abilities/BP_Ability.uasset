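; BP_Ability is an ability base that gates use on the owner's gameplay tags, an overridable final check and a cooldown flag.
; Using it adds tags, flags combat as attacking, changes mana by Cost and plays a montage, undoing tags and flag afterwards.
; It binds an empty apex hook to ABP_Mage's animation dispatcher.
; A mana listener tags depletion at zero, then regenerates mana in a delayed loop.
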(event Custom|UseAblilityPreStep
  ;[0 0 0] A step before using ability, for things like adding tags or other pre ability funtionality
  (for _array_element (Variables|TagFunctionality|GetUseAddingTags)
    (CallFunction|AddAbilityTag _array_element))
  (CallFunction|UseAbility)
  (CallFunction|BindDispatchers))

(event Custom|EndAbility
  ;[0 0 0] undo everything that needs to be undone after using an ability
  (Variables|/Game/Blueprints/Combat/BPC_Combat.BPC_Combat_C|SetAttacking (Variables|Default|GetBPC_Combat) false)
  (for _array_element (Variables|TagFunctionality|GetUseAddingTags)
    (CallFunction|RemoveAbilityTag _array_element)
    (CallFunction|RemoveDispatchers)))

(event Custom|ManaChanged
  (params (AttributeContext :type S%20Attribute%20Context%20Structure))
  (bind (_attributechanged _origin) (Utilities|Struct|BreakS_AttributeContext AttributeContext))
  (bind _returnvalue (Components|GetOwner))
  (bind _basevalue (Utilities|Struct|BreakS_Attribute _attributechanged))
  (bind _returnvalue_2 (Actor|GetComponentbyClass _returnvalue "/Game/Blueprints/GamePlayTags/BPC_GameplayTags.BPC_GameplayTags_C"))
  (if (<= _basevalue 0.0)
    (Default|AddTag _returnvalue_2 "(TagName=\"State.Depleated\")" _origin)
    (if (<= _basevalue 0.0)
      (Utilities|FlowControl|Delay 3.0)
      (Default|ChangeAttribute (Actor|GetComponentbyClass (Components|GetOwner) "/Game/Blueprints/Attributes/BPC_Attributes.BPC_Attributes_C") "(TagName=\"Attribute.Mana\")" 1e+01 "NewEnumerator1" _origin :!label _label)
      (Utilities|FlowControl|Delay 1.0)
      (if (== _basevalue 1e+02)
        (Default|RemoveTag _returnvalue_2 "(TagName=\"State.Depleated\")" _origin)
        (else
          (goto _label))))))

(event Custom|BindDispatchers
  (bind _skeletalmesh (Class|BPIGetMesh|GetMesh(Message) (Components|GetOwner)))
  (bind _asabp_mage (Utilities|Casting|CastToABP_Mage (Components|SkeletalMesh|GetAnimInstance _skeletalmesh)))
  (EventDispatchers|BindEventtoAnimationApexDispatcher _asabp_mage (delegate Custom|AnimationApexEvent)))

(event Custom|AnimationApexEvent)

(event Custom|RemoveDispatchers
  (bind _skeletalmesh (Class|BPIGetMesh|GetMesh(Message) (Components|GetOwner)))
  (bind _asabp_mage (Utilities|Casting|CastToABP_Mage (Components|SkeletalMesh|GetAnimInstance _skeletalmesh)))
  (EventDispatchers|UnbindallEventsfromAnimationApexDispatcher _asabp_mage))

(event Custom|AttemptUseAbility
  (bind _canuseability (CallFunction|CanUseAbility?))
  (if _canuseability
    (CallFunction|UseAblilityPreStep)))

(event Custom|UseAbility
  (bind _returnvalue (Components|GetOwner))
  (bind _returnvalue_2 (Actor|GetComponentbyClass _returnvalue "/Game/Blueprints/Combat/BPC_Combat.BPC_Combat_C"))
  ;[0 0 0] Play motage if applicable
  (Variables|Default|SetBPC_Combat _returnvalue_2)
  (Variables|/Game/Blueprints/Combat/BPC_Combat.BPC_Combat_C|SetAttacking _returnvalue_2 true)
  (Default|ChangeAttribute (Actor|GetComponentbyClass _returnvalue "/Game/Blueprints/Attributes/BPC_Attributes.BPC_Attributes_C") "(TagName=\"Attribute.Mana\")" (Variables|Default|GetCost) "NewEnumerator1")
  (bind _skeletalmesh (Class|BPIGetMesh|GetMesh(Message) _returnvalue))
  (Utilities|IsValid _skeletalmesh
    (:Is%20Valid
      (bind _animationmontage (Variables|Default|GetAnimationMontage)
        (:then
          (Animation|Montage|PlayMontage _skeletalmesh _animationmontage
            (:OnCompleted
              _)
            (:OnInterrupted
              _)))
        (:else
          _)))
    (:Is%20Not%20Valid
      _))
  (CallFunction|EndAbility))

(event EventBeginPlay
  (bind _returnvalue (Components|GetOwner))
  (bind _returnvalue_2 (Actor|GetComponentbyClass _returnvalue "/Game/Blueprints/Attributes/BPC_Attributes.BPC_Attributes_C"))
  (Utilities|IsValid _returnvalue_2
    (:Is%20Valid
      (Default|AddAttributeListener _returnvalue_2 "(TagName=\"Attribute.Mana\")" (delegate Custom|ManaChanged)))))

(fn ConstructionScript)

(fn IsUsingAbilityRestricted
  (bind _returnvalue (Components|GetOwner))
  (bind _returnvalue_2 (Actor|GetComponentbyClass _returnvalue "/Game/Blueprints/GamePlayTags/BPC_GameplayTags.BPC_GameplayTags_C"))
  ;[0 0 0] Check if tags prevent using ability
  (Utilities|IsValid _returnvalue_2
    (:Is%20Valid
      (bind _tagcontainer (Default|GetActiveTagContainer _returnvalue_2))
      (return (GameplayTags|HasAnyTags _tagcontainer (Variables|TagFunctionality|GetUsePreventionTags))))
    (:Is%20Not%20Valid
      (return false))))

(fn IsUsingAbilityPrerequisitesFulfilled?
  (bind _returnvalue (Components|GetOwner))
  (bind _returnvalue_2 (Actor|GetComponentbyClass _returnvalue "/Game/Blueprints/GamePlayTags/BPC_GameplayTags.BPC_GameplayTags_C"))
  (Utilities|IsValid _returnvalue_2
    (:Is%20Valid
      (bind _tagcontainer (Default|GetActiveTagContainer _returnvalue_2))
      (return (GameplayTags|HasAllTags _tagcontainer (Variables|TagFunctionality|GetUseRequiredTags))))
    (:Is%20Not%20Valid
      (return true))))

(fn CanUseAbility?
  ;[0 0 0] Allows character to use ability if nothing is preventing them
  (bind _allowedtouse (CallFunction|FinalUseAllowanceCheck))
  (if _allowedtouse
    ;[0 0 0] Check if tags prevent using ability
    (bind _restricted (CallFunction|IsUsingAbilityRestricted))
    (if _restricted
      (return false)
      (else
        ;[0 0 0] Make sure all required tags are available to use the ability
        (bind _allowed (CallFunction|IsUsingAbilityPrerequisitesFulfilled?))
        (if _allowed
          (if (not (Variables|Default|GetCooldownActivated))
            (return true))
          (else
            (return false)))))
    (else
      (return false))))

(fn AddAbilityTag
  (params (AbilityTag :type Gameplay%20Tag%20Structure))
  (bind _returnvalue (Components|GetOwner))
  (bind _returnvalue_2 (Actor|GetComponentbyClass _returnvalue "/Game/Blueprints/GamePlayTags/BPC_GameplayTags.BPC_GameplayTags_C"))
  ;[0 0 0] Add tags to gameplay component to describe properties effected
  (Utilities|IsValid _returnvalue_2
    (:Is%20Valid
      (Default|AddTag _returnvalue_2 AbilityTag (Utilities|Struct|MakeS_Origin _returnvalue (Game|GetInstigatorController)))
      (return))))

(fn RemoveAbilityTag
  (params (AbilityTag :type Gameplay%20Tag%20Structure))
  (bind _returnvalue (Components|GetOwner))
  (bind _returnvalue_2 (Actor|GetComponentbyClass _returnvalue "/Game/Blueprints/GamePlayTags/BPC_GameplayTags.BPC_GameplayTags_C"))
  ;[0 0 0] Remove tags that were added at the start of the ability
  (Utilities|IsValid _returnvalue_2
    (:Is%20Valid
      (Default|RemoveTag _returnvalue_2 AbilityTag (Utilities|Struct|MakeS_Origin _returnvalue (Game|GetInstigatorController)))
      (return))))

(fn FinalUseAllowanceCheck
  ;[0 0 0] Allows character to use ability if nothing is preventing them
  (return true))
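; Magic projectile ability Blueprint that launches a projectile when the ability's animation reaches its apex.
; The apex event calls FireProjectile on the owner's BPC_Combat component.
; CreateProjectileStats builds the projectile stats, scaling damage from a level curve at the current ability level by a power multiplier and enabling an explosion radius.
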(event EventBeginPlay
  (|CallParentFunction) ; This node is disabled and will not be called.\nDrag off pins to build functionality.
)

(event EventAnimationApexEvent
  (Default|FireProjectile (Actor|GetComponentbyClass (Components|GetOwner) "/Game/Blueprints/Combat/BPC_Combat.BPC_Combat_C")))

(fn ConstructionScript
  (|CallParentFunction))

(fn CreateProjectileStats
  (return (Utilities|Struct|MakeS_ProjectileStats (* (Math|Curves|GetFloatValue (Variables|Default|GetLevelCurve) (Variables|Default|GetCurrentAbilityLevel)) (Variables|Default|GetPowerMultiplier)) 3e+03 (Variables|Default|GetExplosion%20Radius) true)))
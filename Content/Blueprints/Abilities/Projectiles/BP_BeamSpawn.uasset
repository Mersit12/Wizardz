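; BP_BeamSpawn is a beam ability projectile that deals area damage on destruction and supplies a damage segment between its mesh's A and B sockets.
; Its Destruction event damages pawns within the explosion radius using ProjectileStats, reporting damage events for them and the hit actor.
; The single-target damage branch is unreachable behind a hardwired true condition.
; The actor destroys itself after a fixed delay.
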(event EventBeginPlay)

(event Collision|EventActorBeginOverlap
  (params (OtherActor :type Actor%20Object%20Reference)))

(event EventTick
  (params (DeltaSeconds :type Float%20%28single-precision%29)))

(event EventDestruction
  (params (HitActor :type Actor%20Object%20Reference))
  (bind _returnvalue (Game|GetInstigatorController))
  (bind _projectilestats (Variables|Default|GetProjectileStats))
  (bind _damage (Utilities|Struct|BreakS_ProjectileStats _projectilestats))
  (if true
    (if (Variables|Default|GetDrawDebug)
      _
      (else
        _))
    (bind _outactors (Collision|SphereOverlapActors (Transformation|GetActorLocation) (.ExplosionRadius (Utilities|Struct|BreakS_ProjectileStats (Variables|Default|GetProjectileStats))) (Utilities|Array|MakeArray "ObjectTypeQuery3") 0))
    (for _array_element _outactors
      (bind _returnvalue_2 (Game|Damage|ApplyDamage _array_element (.Damage (Utilities|Struct|BreakS_ProjectileStats (Variables|Default|GetProjectileStats))) _returnvalue self))
      (Class|AISenseDamage|ReportDamageEvent _array_element _returnvalue _returnvalue_2 (Transformation|GetActorLocation HitActor) "0, 0, 0" "None"))
    (else
      (Game|Damage|ApplyDamage HitActor _damage (Game|GetInstigatorController) self)))
  (Class|AISenseDamage|ReportDamageEvent HitActor _returnvalue _damage (Transformation|GetActorLocation HitActor) "0, 0, 0" "None")
  (Utilities|FlowControl|Delay 7.67)
  (Actor|DestroyActor))

(fn ConstructionScript
  (|CallParentFunction))

(fn GetDamageLocations
  (bind _staticmesh (Variables|Default|GetStaticMesh))
  (return (Utilities|Array|MakeArray (Utilities|Struct|MakeS_DamageLocations (Transformation|GetSocketLocation _staticmesh "A") (Transformation|GetSocketLocation _staticmesh "B")))))
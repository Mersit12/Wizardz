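; BP_SpinningAxe is an axe ability projectile that spins and destroys itself three seconds after BeginPlay.
; A looping timeline drives the scene component's world yaw, restarting through the SpinAxe event.
; The first skeletal mesh overlap, if not with the owner, calls Destruction on that actor and spawns a hit effect and metal impact sound.
; DoOnce precedes the owner check, so an owner overlap also consumes it.
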(event OnComponentBeginOverlap(SkeletalMesh)
  (params (OverlappedComponent :type Primitive%20Component%20Object%20Reference) (OtherActor :type Actor%20Object%20Reference) (OtherComp :type Primitive%20Component%20Object%20Reference) (OtherBodyIndex :type Integer) (bFromSweep :type Boolean) (SweepResult :type Hit%20Result%20Structure%20%28by%20ref%29))
  (bind _returnvalue (Transformation|GetActorLocation OtherActor))
  (Utilities|FlowControl|DoOnce false
    (:Completed
      (if (!= OtherActor (Components|GetOwner))
        (CallFunction|Destruction OtherActor)
        (Niagara|SpawnSystematLocation "/Game/VFX/WizardSpellsPack/sA_Megapack_v1/sA_StylizedAttacksPack/FX/NiagaraSystems/NS_BasicHit.NS_BasicHit" _returnvalue)
        (Audio|PlaySoundatLocation "/Game/SoundFX/Free_Sounds_Pack/Shield_Metal_Impact_1-3.Shield_Metal_Impact_1-3" _returnvalue "0, 0, 0" 1.0 1.0 0.0 0 0 0 0)))))

(event Custom|SpinAxe
  (bind _scene (Variables|Default|GetScene))
  (bind _returnvalue (Transformation|GetWorldRotation _scene))
  (bind _zrotation (Timeline|RotationTimeline PlayFromStart)
    (:Update
      (Transformation|SetWorldRotation (Variables|Default|GetScene) (Math|Rotator|MakeRotator (.roll _returnvalue) (.pitch _returnvalue) _zrotation) false false))
    (:Finished
      (CallFunction|SpinAxe))))

(event EventBeginPlay
  (|CallParentFunction)
  (CallFunction|SpinAxe)
  (Utilities|FlowControl|Delay 3.0)
  (Actor|DestroyActor))

(event Collision|EventActorBeginOverlap
  (params (OtherActor :type Actor%20Object%20Reference)))

(event EventTick
  (params (DeltaSeconds :type Float%20%28single-precision%29)))

(event Collision|EventHit
  (params (MyComp :type Primitive%20Component%20Object%20Reference) (Other :type Actor%20Object%20Reference) (OtherComp :type Primitive%20Component%20Object%20Reference) (bSelfMoved :type Boolean) (HitLocation :type Vector :default "0, 0, 0") (HitNormal :type Vector :default "0, 0, 0") (NormalImpulse :type Vector :default "0, 0, 0") (Hit :type Hit%20Result%20Structure%20%28by%20ref%29))
  (|CallParentFunction MyComp Other OtherComp bSelfMoved HitLocation HitNormal NormalImpulse Hit))

(fn ConstructionScript
  (|CallParentFunction))
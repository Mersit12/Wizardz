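; BP_ProjectileBase is an ability projectile base that deals damage on impact and then destroys itself.
; Mesh overlaps with anything but the owner, and any Hit event, feed a shared Destruction event.
; Driven by ProjectileStats, it damages either the struck actor or every Pawn in the explosion radius, crediting the instigator's controller.
; The radial sphere query has an optional debug draw and does not exclude the owner.
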(event OnComponentBeginOverlap(StaticMesh)
  (params (OverlappedComponent :type Primitive%20Component%20Object%20Reference) (OtherActor :type Actor%20Object%20Reference) (OtherComp :type Primitive%20Component%20Object%20Reference) (OtherBodyIndex :type Integer) (bFromSweep :type Boolean) (SweepResult :type Hit%20Result%20Structure%20%28by%20ref%29))
  (if (!= OtherActor (Components|GetOwner))
    (CallFunction|Destruction OtherActor)))

(event Custom|Destruction
  (params (HitActor :type Actor%20Object%20Reference))
  (bind _projectilestats (Variables|Default|GetProjectileStats))
  (if (Utilities|Struct|BreakS_ProjectileStats _projectilestats)
    (if (Variables|Default|GetDrawDebug)
      (Rendering|Debug|DrawDebugSphere (Transformation|GetActorLocation) (Utilities|Struct|BreakS_ProjectileStats (Variables|Default|GetProjectileStats)) 12 "(R=1.000000,G=0.000000,B=0.026704,A=1.000000)" 5.0 1.0))
    (bind _outactors (Collision|SphereOverlapActors (Transformation|GetActorLocation) (Utilities|Struct|BreakS_ProjectileStats (Variables|Default|GetProjectileStats)) (Utilities|Array|MakeArray "ObjectTypeQuery3") 0))
    (for _array_element _outactors
      (Game|Damage|ApplyDamage _array_element (Utilities|Struct|BreakS_ProjectileStats (Variables|Default|GetProjectileStats)) (Game|GetInstigatorController) self))
    (else
      (Game|Damage|ApplyDamage HitActor (Utilities|Struct|BreakS_ProjectileStats _projectilestats) (Game|GetInstigatorController) self)))
  (Actor|DestroyActor))

(event EventBeginPlay)

(event Collision|EventHit
  (params (MyComp :type Primitive%20Component%20Object%20Reference) (Other :type Actor%20Object%20Reference) (OtherComp :type Primitive%20Component%20Object%20Reference) (bSelfMoved :type Boolean) (HitLocation :type Vector :default "0, 0, 0") (HitNormal :type Vector :default "0, 0, 0") (NormalImpulse :type Vector :default "0, 0, 0") (Hit :type Hit%20Result%20Structure%20%28by%20ref%29))
  (CallFunction|Destruction Other))

(fn ConstructionScript)
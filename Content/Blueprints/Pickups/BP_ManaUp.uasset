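; BP_ManaUp is a pickup that gives the third-person player character a BP_StatusEffects_ManaDrop status effect on overlap.
; Its trigger spawns the effect actor owned by the player and registers it with the character's BPCStatusEffects component.
; It then spawns an activation particle system and, after a delay, destroys both the particles and itself.
; Nothing disables the trigger during that delay, so repeat overlaps can apply further effects.
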(event OnComponentBeginOverlap(PickupTrigger)
  (params (OverlappedComponent :type Primitive%20Component%20Object%20Reference) (OtherActor :type Actor%20Object%20Reference) (OtherComp :type Primitive%20Component%20Object%20Reference) (OtherBodyIndex :type Integer) (bFromSweep :type Boolean) (SweepResult :type Hit%20Result%20Structure%20%28by%20ref%29))
  (bind _asbp_third_person_character (Utilities|Casting|CastToBP_ThirdPersonCharacter OtherActor))
  (Variables|Default|SetPlayerREF _asbp_third_person_character)
  (bind _returnvalue (Game|SpawnActorfromClass :Class "/Game/Blueprints/StatusEffects/Buffs/BP_StatusEffects_ManaDrop.BP_StatusEffects_ManaDrop_C" :SpawnTransform (Transformation|GetActorTransform self) :CollisionHandlingOverride "AlwaysSpawn" :TransformScaleMethod "OverrideRootScale" :Owner _asbp_third_person_character :Instigator 0))
  (Default|AddStatusEffect (Variables|/Game/ThirdPerson/Blueprints/BP_ThirdPersonCharacter.BP_ThirdPersonCharacter_C|GetBPC_StatusEffects (Variables|Default|GetPlayerREF)) _returnvalue)
  (bind _returnvalue_2 (Niagara|SpawnSystematLocation (Variables|Default|GetActivationSystem) (Transformation|GetActorLocation self)))
  (Utilities|FlowControl|Delay 6.0)
  (Components|DestroyComponent _returnvalue_2)
  (Actor|DestroyActor))

(event EventBeginPlay
  (|CallParentFunction) ; This node is disabled and will not be called.\nDrag off pins to build functionality.
)

(event Collision|EventActorBeginOverlap
  (params (OtherActor :type Actor%20Object%20Reference))
  (|CallParentFunction OtherActor) ; This node is disabled and will not be called.\nDrag off pins to build functionality.
)

(event EventTick
  (params (DeltaSeconds :type Float%20%28single-precision%29))
  (|CallParentFunction DeltaSeconds) ; This node is disabled and will not be called.\nDrag off pins to build functionality.
)

(fn ConstructionScript
  (|CallParentFunction))
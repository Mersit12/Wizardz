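; BPC_XP is an actor component that tracks experience and levels and awards XP to the killer when its owner dies.
; It listens for the State.Dead tag on the owner's BPC_GameplayTags, then calls AwardXP on the BPC_XP of the origin controller's pawn.
; AwardXP checks LevelCurve recursively for multiple level-ups up to MaxLevel, firing LevelUp for each, then XPChanged, whose context always reports level 0.
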(event Custom|DeadStateUpdated
  (params (GameplayTagContext :type S%20Gameplay%20Context%20Structure))
  (bind (_contexttag _activetags _origin) (Utilities|Struct|BreakS_GameplayContext GameplayTagContext))
  (bind _controller (Utilities|Struct|BreakS_Origin _origin))
  (bind _returnvalue (Pawn|GetControlledPawn _controller))
  (bind _returnvalue_2 (Actor|GetComponentbyClass _returnvalue "BPC_XP_C"))
  ;[0 0 0] Check if we are dead
  (if (GameplayTags|HasTag _activetags "(TagName=\"State.Dead\")")
    ;[0 0 0] We are dead. Award XP to our killer
    (Utilities|IsValid _controller
      (:Is%20Valid
        (Utilities|IsValid _returnvalue
          (:Is%20Valid
            (Utilities|IsValid _returnvalue_2
              (:Is%20Valid
                (CallFunction|AwardXP _returnvalue_2 (Variables|Default|GetXPToAward))))))))))

(event Custom|AwardXP
  (params (AwardedXP :type Float%20%28double-precision%29))
  ;[0 0 0] Adds an XP amount and tries to level up if possible
  (bind _output_get (Variables|Default|SetCurrentXP (+ (Variables|Default|GetCurrentXP) AwardedXP)))
  (CallFunction|TrytoLevelUp)
  ;[0 0 0] Inform that XP has changed
  (Default|CallXPChanged (Utilities|Struct|MakeS_XPContext _output_get 0 AwardedXP)))

(event Custom|Signature
  (params (XPContext :type S%20XP%20Context%20Structure))
  ;[0 0 0] Placeholder dummy for signature for event dispatchers
)

(event EventBeginPlay
  (bind _returnvalue (Components|GetOwner))
  (bind _returnvalue_2 (Actor|GetComponentbyClass _returnvalue "/Game/Blueprints/GamePlayTags/BPC_GameplayTags.BPC_GameplayTags_C"))
  (Utilities|IsValid _returnvalue_2
    (:Is%20Valid
      ;[0 0 0] Listen if owner dies
      (Default|AddTagListener _returnvalue_2 "(TagName=\"State.Dead\")" (delegate Custom|DeadStateUpdated)))))

(fn LevelUp?
  ;[0 0 0] Check if we aremax level
  (if (== (Variables|Default|GetCurrentLevel) (Variables|Default|GetMaxLevel))
    ;[0 0 0] We are max level
    (return false)
    (elif (>= (Variables|Default|GetCurrentXP) (Math|Curves|GetFloatValue (Variables|Default|GetLevelCurve) (Math|Conversions|ToFloat(Integer) (+ (Variables|Default|GetCurrentLevel) 1))))
      ;[0 0 0] Levelled up
      (Math|Integer|IncrementInt (Variables|Default|GetCurrentLevel)
        (:%20%20
          (return true)))
      (else
        ;[0 0 0] Not enough XP
        (return false)))))

(fn TrytoLevelUp
  ;[0 0 0] Check if we surpassed a level up threshold
  (bind _levelledup (CallFunction|LevelUp?))
  (if _levelledup
    ;[0 0 0] Did level up. Inform we levelled up
    (Default|CallLevelUp (Utilities|Struct|MakeS_XPContext (Variables|Default|GetCurrentXP) (Variables|Default|GetCurrentLevel) 0.0))
    ;[0 0 0] Check to see if there are multiple level ups
    (CallFunction|TrytoLevelUp)
    (return)
    (else
      ;[0 0 0] Did not level up
      (return))))

(fn ResetLevel
  (Variables|Default|SetCurrentLevel 1))
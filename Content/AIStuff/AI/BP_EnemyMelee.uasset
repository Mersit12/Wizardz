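; Melee enemy Blueprint that handles sword attacks and drawing or sheathing the sword.
; Equip and unequip go through BPCCombat, then play montages whose notifies toggle IsWieldingWeapon.
; Event dispatchers report when each action ends: attack on completion or interruption, equip and unequip only on completion.
; GetSpellSpawnLocation and GetPatrolRoute are empty stubs.
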(event EventBeginPlay
  (|CallParentFunction) ; This node is disabled and will not be called.\nDrag off pins to build functionality.
)

(event EventEquipWeapon
  (Default|EquipWeapon (Variables|Default|GetBPC_Combat) "/Game/Blueprints/Weapons/BP_Sword.BP_Sword_C" "SwordSocket")
  (Animation|Montage|PlayMontage (Variables|Character|GetMesh) "/Game/AIStuff/Animations/Melee/Montage_Unsheath_Sword.Montage_Unsheath_Sword"
    (:OnCompleted
      (Default|CallOnWeaponEquipped))
    (:OnNotifyBegin
      (Variables|Default|SetIsWieldingWeapon true))))

(event EventUnequipWeapon
  (Default|UnequipWeapon (Variables|Default|GetBPC_Combat))
  (Animation|Montage|PlayMontage (Variables|Character|GetMesh) "/Game/AIStuff/Animations/Melee/Montage_Sheath_Sword.Montage_Sheath_Sword"
    (:OnCompleted
      (Default|CallOnWeaponEnequipped))
    (:OnNotifyBegin
      (Variables|Default|SetIsWieldingWeapon false))))

(event EventAttack
  (Animation|Montage|PlayMontage (Variables|Character|GetMesh) "/Game/AIStuff/Animations/Melee/Montage_Sword_Slash.Montage_Sword_Slash"
    (:OnCompleted
      _)
    (:OnInterrupted
      _))
  (Default|CallOnAttackEnd))

(fn ConstructionScript
  (|CallParentFunction))

(fn GetSpellSpawnLocation
  (return ""))

(fn GetPatrolRoute
  (return 0))
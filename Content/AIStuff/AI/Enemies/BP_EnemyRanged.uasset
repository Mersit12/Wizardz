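; Ranged enemy character that equips a crossbow on spawn and fights from a fixed ideal range, extending a parent enemy class.
; Attack plays a rifle fire montage, whose notify traces from the SpellSpawner to the target and applies hitscan damage through BPCCombat if unobstructed.
; Montage completion or interruption ends the attack, followed by a delayed sound.
; Overrides supply movement speeds and attack and defend radii.
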(event EventBeginPlay
  (|CallParentFunction)
  (CallFunction|EquipWeapon))

(event EventEquipWeapon
  (Default|EquipWeapon (Variables|Default|GetBPC_Combat) "/Game/Blueprints/Weapons/BP_Crossbow.BP_Crossbow_C" "RifleSocket")
  (Variables|Default|SetIsWieldingWeapon true)
  (Default|CallOnWeaponEquipped))

(event EventAttack
  (params (AttackTarget :type Actor%20Object%20Reference))
  (|CallParentFunction AttackTarget)
  (bind _notifyname (Animation|Montage|PlayMontage (Variables|Character|GetMesh) "/Game/AIStuff/Animations/Rifle/Montage_Rifle_Fire.Montage_Rifle_Fire")
    (:OnCompleted
      (CallFunction|AttackEnd AttackTarget :!label _label)
      (Utilities|FlowControl|Delay 1.0)
      (Audio|PlaySoundatLocation "/Engine/VREditor/Sounds/UI/Gizmo_Handle_Clicked.Gizmo_Handle_Clicked" (Transformation|GetActorLocation) "0, 0, 0" 1.2 1.0 0.0 0 0 0 0))
    (:OnInterrupted
      (goto _label))
    (:OnNotifyBegin
      (switch name _notifyname
        (:Fire
          (bind _spellspawntransform (CallFunction|GetSpellSpawnLocation))
          (bind _returnvalue (Collision|LineTraceByChannel (.location _spellspawntransform) (Transformation|GetActorLocation AttackTarget) "TraceTypeQuery1" false 0 "None"))
          (if (not _returnvalue)
            (Default|DamageTaken (Variables|Default|GetBPC_Combat) AttackTarget (Variables|Default|GetDamage) 0 (AI|GetAIController self) self)))))))

(fn ConstructionScript
  (|CallParentFunction))

(fn SetMovementSpeed
  (params (Speed :type E_MovementSpeed%20Enum :default "NewEnumerator0"))
  (Variables|/Script/Engine.CharacterMovementComponent|SetMaxWalkSpeed (Variables|Character|GetCharacterMovement) (Utilities|Select :Index Speed :NewEnumerator0 0.0 :NewEnumerator1 2e+02 :NewEnumerator2 2.5e+02 :NewEnumerator3 4e+02))
  (return 0.0))

(fn GetIdealRange
  (return 6e+02 6e+02))

(fn GetSpellSpawnLocation
  (return (Transformation|GetWorldTransform (Variables|Default|GetSpellSpawner))))
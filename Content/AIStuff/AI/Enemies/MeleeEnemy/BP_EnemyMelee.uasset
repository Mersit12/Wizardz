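; Sword-wielding melee enemy character that supplies its attacks, weapon handling and AI tuning values.
; Short, spinning, long-range jump and ground smash attacks each pass a target and montage to the BPCCombat component.
; Equip and unequip play sheath montages, toggling the wielding flag on notify and firing dispatchers on completion.
; Query functions provide movement speeds, ideal combat ranges, team number and velocity-predicted locations, while spell spawn and patrol route are empty.
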(event Custom|ShortRangedAttack
  (params (AttackTarget :type Actor%20Object%20Reference))
  (Default|PrimaryMeleeAttack (Variables|Default|GetBPC_Combat) (Utilities|Struct|MakeS_AttackInfo AttackTarget "/Game/Montage_Sword_Slash.Montage_Sword_Slash")))

(event Custom|SpinningAttack
  (params (AttackTarget :type Actor%20Object%20Reference))
  (Default|SpinningMeleeAttack (Variables|Default|GetBPC_Combat) (Utilities|Struct|MakeS_AttackInfo AttackTarget "/Game/AIStuff/Animations/SkeletonMelee/Montage_Sword_SpinningAttack.Montage_Sword_SpinningAttack")))

(event Custom|LongRangedAttack
  (params (AttackTarget :type Actor%20Object%20Reference))
  (Default|LongRangedMeleeAttack (Variables|Default|GetBPC_Combat) (Utilities|Struct|MakeS_AttackInfo AttackTarget "/Game/AIStuff/Animations/Melee/Montage_Sword_Jump_Attack.Montage_Sword_Jump_Attack")))

(event Custom|GroundSmashAttack
  (params (AttackTarget :type Actor%20Object%20Reference))
  (Default|GroundSmashAttack (Variables|Default|GetBPC_Combat) (Utilities|Struct|MakeS_AttackInfo AttackTarget "/Game/AIStuff/Animations/SkeletonMelee/Montage_Melee_GroundSmash.Montage_Melee_GroundSmash") 3e+02 5e+01))

(event EventBeginPlay
  (|CallParentFunction) ; This node is disabled and will not be called.\nDrag off pins to build functionality.
)

(event EventEquipWeapon
  (Default|EquipWeapon (Variables|Default|GetBPC_Combat) "/Game/Blueprints/Weapons/BP_Sword.BP_Sword_C" "SwordSocket")
  (Animation|Montage|PlayMontage (Variables|Character|GetMesh) "/Game/AIStuff/Animations/Melee/Montage_Unsheath_Sword.Montage_Unsheath_Sword"
    (:OnCompleted
      (Default|CallOnWeaponEquipped))
    (:OnNotifyBegin
      (Variables|Default|SetIsWieldingWeapon true))))

(event EventUnequipWeapon
  (Default|UnequipWeapon (Variables|Default|GetBPC_Combat))
  (Animation|Montage|PlayMontage (Variables|Character|GetMesh) "/Game/AIStuff/Animations/Melee/Montage_Sheath_Sword.Montage_Sheath_Sword"
    (:OnCompleted
      (Default|CallOnWeaponEnequipped))
    (:OnNotifyBegin
      (Variables|Default|SetIsWieldingWeapon false))))

(fn ConstructionScript
  (|CallParentFunction)
  (Variables|Default|SetMeshRotationBeforeSpin (Variables|/Script/Engine.SceneComponent|GetRelativeRotation (Variables|Character|GetMesh))))

(fn GetSpellSpawnLocation
  (return ""))

(fn GetPatrolRoute
  (return 0))

(fn SetMovementSpeed
  (params (Speed :type E_MovementSpeed%20Enum :default "NewEnumerator0"))
  (bind _output_get (Variables|/Script/Engine.CharacterMovementComponent|SetMaxWalkSpeed (Variables|Character|GetCharacterMovement) (Utilities|Select :Index Speed :NewEnumerator0 0.0 :NewEnumerator1 1.5e+02 :NewEnumerator2 2.5e+02 :NewEnumerator3 4e+02)))
  (return _output_get))

(fn GetIdealRange
  (return 2e+02 4e+02))

(fn CalculateFutureActorLocation
  (params (Actor :type Actor%20Object%20Reference) (Time :type Float%20%28double-precision%29))
  (return (+ (Transformation|GetActorLocation Actor) (* (* (Transformation|GetVelocity Actor) "1.000000,1.000000,0.000000") Time))))

(fn GetTeamNumber
  (return 1))
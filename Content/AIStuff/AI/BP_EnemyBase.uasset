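; Base enemy character Blueprint that takes damage, reacts to hits and answers queries from its AI.
; AnyDamage subtracts from the health attribute through BPCAttributes, then freezes the owning BP_EnemyAIController during a hit montage and switches it to attacking the player afterwards.
; Getter functions supply combat ranges, patrol route, mesh, spell spawn transforms and team number.
; SetMovementSpeed maps movement states to walk speeds, while ReserveAttackToken is a stub returning false.
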(event Custom|HitReaction
  (bind _asbp_enemy_aicontroller (Utilities|Casting|CastToBP_EnemyAIController (Components|GetOwner)))
  (Default|SetStateasFrozen _asbp_enemy_aicontroller)
  (Animation|Montage|PlayMontage (Variables|Character|GetMesh) (Variables|Default|GetHitMontage)
    (:OnCompleted
      _)
    (:OnInterrupted
      _))
  (Default|SetStateasAttacking _asbp_enemy_aicontroller (Game|GetPlayerCharacter 0)))

(event EventBeginPlay)

(event Game|Damage|EventAnyDamage
  (params (Damage :type Float%20%28single-precision%29) (DamageType :type Damage%20Type%20Object%20Reference) (InstigatedBy :type Controller%20Object%20Reference) (DamageCauser :type Actor%20Object%20Reference))
  (Default|ChangeAttribute (Variables|Default|GetBPC_Attributes) "(TagName=\"Attribute.Health\")" (* Damage -1.0) "NewEnumerator1" (Utilities|Struct|MakeS_Origin InstigatedBy (Game|GetPlayerController 0)))
  (CallFunction|HitReaction))

(fn ConstructionScript)

(fn GetIdealRange
  (return 1.5e+02 3.5e+02))

(fn GetMesh
  (return (Variables|Character|GetMesh)))

(fn GetPatrolRoute
  (return (Variables|AI|GetPatrolRoute)))

(fn GetSpellSpawnLocation
  (return (Transformation|GetWorldTransform (Variables|Default|GetSpellSpawner))))

(fn GetStantionarySpawnLocation
  (return (Transformation|GetWorldTransform (Variables|Default|GetStationarySpellSpawner))))

(fn GetTeamNumber
  (return 0))

(fn ReserveAttackToken
  (params (Amount :type Integer))
  (return false))

(fn SetMovementSpeed
  (params (Speed :type E_MovementSpeed%20Enum :default "NewEnumerator0"))
  (bind _output_get (Variables|/Script/Engine.CharacterMovementComponent|SetMaxWalkSpeed (Variables|Character|GetCharacterMovement) (Utilities|Select :Index Speed :NewEnumerator0 0.0 :NewEnumerator1 1e+02 :NewEnumerator2 2.5e+02 :NewEnumerator3 4e+02)))
  (return _output_get))
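; BP_EnemyMage is a ranged spellcasting enemy that attacks through an ability component.
; BeginPlay initializes BPCAbility with its ability list, and each Attack fires ability index 0, then immediately calls AttackEnd.
; It overrides movement speeds per state and its ideal attack and defend ranges.
; Two spawner components supply world transforms for regular and stationary spell spawn points.
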(event EventBeginPlay
  (|CallParentFunction)
  (Default|InitializeAbilities (Variables|Default|GetBPC_Ability) (Variables|Default|GetAbilities)))

(event EventAttack
  (params (AttackTarget :type Actor%20Object%20Reference))
  (|CallParentFunction AttackTarget)
  (Default|UseAbility (Variables|Default|GetBPC_Ability))
  (CallFunction|AttackEnd AttackTarget))

(fn ConstructionScript
  (|CallParentFunction))

(fn SetMovementSpeed
  (params (Speed :type E_MovementSpeed%20Enum :default "NewEnumerator0"))
  (return (Utilities|Select :Index Speed :NewEnumerator0 0.0 :NewEnumerator1 1.5e+02 :NewEnumerator2 2.5e+02 :NewEnumerator3 4e+02)))

(fn GetIdealRange
  (return 5e+02 7e+02))

(fn GetSpellSpawnLocation
  (return (Transformation|GetWorldTransform (Variables|Default|GetSpellSpawner))))

(fn GetStantionarySpawnLocation
  (return (Transformation|GetWorldTransform (Variables|Default|GetStationarySpellSpawner))))
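; Ranged enemy character that overrides its parent's equip, attack, movement speed and ideal range behavior for crossbow combat.
; On BeginPlay it equips a crossbow through the combat component, and Attack plays a rifle fire montage that signals attack end on completion or interruption.
; A montage notify runs a debug line trace from the spell spawner toward the target, only printing a message when unblocked, with no projectile or damage.
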(event EventBeginPlay
  (CallFunction|EquipWeapon))

(event EventEquipWeapon
  (Default|EquipWeapon (Variables|Default|GetBPC_Combat) "/Game/Blueprints/Weapons/BP_Crossbow.BP_Crossbow_C" "RifleSocket")
  (Variables|Default|SetIsWieldingWeapon true)
  (Default|CallOnWeaponEquipped))

(event EventAttack
  (bind _notifyname (Animation|Montage|PlayMontage (Variables|Character|GetMesh) "/Game/AIStuff/Animations/Rifle/Montage_Rifle_Fire.Montage_Rifle_Fire")
    (:OnCompleted
      (Default|CallOnAttackEnd :!label _label))
    (:OnInterrupted
      (goto _label))
    (:OnNotifyBegin
      (switch name _notifyname
        (:Fire
          (bind _asbp_enemy_aicontroller (Utilities|Casting|CastToBP_EnemyAIController (AI|GetAIController self)))
          (bind _output_get (Variables|Default|SetAttackTarget _asbp_enemy_aicontroller))
          (bind _spellspawntransform (CallFunction|GetSpellSpawnLocation))
          (bind _returnvalue (Collision|LineTraceByChannel (.location _spellspawntransform) (Transformation|GetActorLocation _output_get) "TraceTypeQuery1" false (Utilities|Array|MakeArray self) "ForDuration"))
          (if (not _returnvalue)
            (Development|PrintString "HIT TAa")))))))

(fn ConstructionScript
  (|CallParentFunction))

(fn SetMovementSpeed
  (params (Speed :type E_MovementSpeed%20Enum :default "NewEnumerator0"))
  (Variables|/Script/Engine.CharacterMovementComponent|SetMaxWalkSpeed (Variables|Character|GetCharacterMovement) (Utilities|Select :Index Speed :NewEnumerator0 0.0 :NewEnumerator1 2e+02 :NewEnumerator2 2.5e+02 :NewEnumerator3 4e+02))
  (return 0.0))

(fn GetIdealRange
  (return 6e+02 6e+02))

(fn GetSpellSpawnLocation
  (return (Transformation|GetWorldTransform (Variables|Default|GetSpellSpawner))))
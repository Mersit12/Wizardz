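; BP_RoomTrigger is a trigger volume that activates enemy spawn rooms when a BP_ThirdPersonCharacter overlaps it.
; On overlap it caches the player and the level's BP_WaveManager, then loops through all of the manager's EnemySpawnPoints.
; Each point gets an active tag matching its own RoomID, and the manager's matching OnEnterRoom function is called once per point.
; The trigger applies no room filter of its own, and end overlap does nothing.
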(event OnComponentBeginOverlap(Trigger)
  (params (OverlappedComponent :type Primitive%20Component%20Object%20Reference) (OtherActor :type Actor%20Object%20Reference) (OtherComp :type Primitive%20Component%20Object%20Reference) (OtherBodyIndex :type Integer) (bFromSweep :type Boolean) (SweepResult :type Hit%20Result%20Structure%20%28by%20ref%29))
  (bind _asbp_third_person_character (Utilities|Casting|CastToBP_ThirdPersonCharacter OtherActor))
  (Variables|Default|SetPlayerREF _asbp_third_person_character)
  (bind _returnvalue (Actor|GetActorOfClass "/Game/AIStuff/Spawner/BP_WaveManager.BP_WaveManager_C"))
  (Variables|Default|SetWaveManagerREF _returnvalue)
  (for _array_element (Variables|/Game/AIStuff/Spawner/BP_WaveManager.BP_WaveManager_C|GetEnemySpawnPoints _returnvalue)
    (switch Utilities|FlowControl|Switch|SwitchonE_Rooms (Variables|/Game/AIStuff/Spawner/BP_WaveSpawnPoint.BP_WaveSpawnPoint_C|GetRoomID _array_element)
      (:NewEnumerator0
        (Utilities|Array|Add (Variables|/Script/Engine.Actor|GetTags _array_element) "Room1Active")
        (Default|OnEnterRoom1 (Variables|Default|GetWaveManagerREF)))
      (:NewEnumerator1
        (Utilities|Array|Add (Variables|/Script/Engine.Actor|GetTags _array_element) "Room2Active")
        (Default|OnEnterRoom2 (Variables|Default|GetWaveManagerREF)))
      (:NewEnumerator2
        (Utilities|Array|Add (Variables|/Script/Engine.Actor|GetTags _array_element) "Room3Active")
        (Default|OnEnterRoom3 (Variables|Default|GetWaveManagerREF)))
      (:NewEnumerator3
        (Utilities|Array|Add (Variables|/Script/Engine.Actor|GetTags _array_element) "Room4Active")
        (Default|OnEnterRoom4 (Variables|Default|GetWaveManagerREF))))))

(event OnComponentEndOverlap(Trigger)
  (params (OverlappedComponent :type Primitive%20Component%20Object%20Reference) (OtherActor :type Actor%20Object%20Reference) (OtherComp :type Primitive%20Component%20Object%20Reference) (OtherBodyIndex :type Integer)))

(event EventBeginPlay)

(event Collision|EventActorBeginOverlap
  (params (OtherActor :type Actor%20Object%20Reference)))

(event EventTick
  (params (DeltaSeconds :type Float%20%28single-precision%29)))

(fn ConstructionScript)
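; BP_Dungeon_Doorway is a double dungeon door that swings open when a player enters its trigger box and closes when they leave.
; Overlapping actors must implement BPI_Player, and the Locked flag blocks opening only.
; One timeline per leaf lerps yaw a quarter turn in opposite directions, reversing to close.
; Rotation is set in world space, so the swing ignores the placed actor's orientation.
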(event OnComponentBeginOverlap(Box)
  (params (OverlappedComponent :type Primitive%20Component%20Object%20Reference) (OtherActor :type Actor%20Object%20Reference) (OtherComp :type Primitive%20Component%20Object%20Reference) (OtherBodyIndex :type Integer) (bFromSweep :type Boolean) (SweepResult :type Hit%20Result%20Structure%20%28by%20ref%29))
  (if (not (Variables|Default|GetLocked))
    (if (Utilities|DoesObjectImplementInterface OtherActor "/Game/Blueprints/Interfaces/BPI_Player.BPI_Player_C")
      (CallFunction|AnimateDoors))))

(event OnComponentEndOverlap(Box)
  (params (OverlappedComponent :type Primitive%20Component%20Object%20Reference) (OtherActor :type Actor%20Object%20Reference) (OtherComp :type Primitive%20Component%20Object%20Reference) (OtherBodyIndex :type Integer))
  (if (Utilities|DoesObjectImplementInterface OtherActor "/Game/Blueprints/Interfaces/BPI_Player.BPI_Player_C")
    (CallFunction|CloseDoors)))

(event Custom|OpenDoorRight
  (bind _rotatetrack (Timeline|Timeline Play)
    (:Update
      (Transformation|SetWorldRotation (Variables|Default|GetSM_DoorWay_Large_Door_Right) (Math|Rotator|MakeRotator 0.0 0.0 (Math|Float|Lerp 0.0 9e+01 _rotatetrack)) false false))))

(event Custom|CloseDoorRight
  (bind _rotatetrack (Timeline|Timeline Reverse)
    (:Update
      (Transformation|SetWorldRotation (Variables|Default|GetSM_DoorWay_Large_Door_Right) (Math|Rotator|MakeRotator 0.0 0.0 (Math|Float|Lerp 0.0 9e+01 _rotatetrack)) false false))))

(event Custom|AnimateDoors
  (CallFunction|OpenDoorLeft)
  (CallFunction|OpenDoorRight))

(event Custom|OpenDoorLeft
  (bind _rotatetrack (Timeline|RotateDoorLeftTimeline Play)
    (:Update
      (Transformation|SetWorldRotation (Variables|Default|GetSM_DoorWay_Large_Door_Left) (Math|Rotator|MakeRotator 0.0 0.0 (Math|Float|Lerp 0.0 -9e+01 _rotatetrack)) false false))))

(event Custom|CloseDoorLeft
  (bind _rotatetrack (Timeline|RotateDoorLeftTimeline Reverse)
    (:Update
      (Transformation|SetWorldRotation (Variables|Default|GetSM_DoorWay_Large_Door_Left) (Math|Rotator|MakeRotator 0.0 0.0 (Math|Float|Lerp 0.0 -9e+01 _rotatetrack)) false false))))

(event Custom|CloseDoors
  (CallFunction|CloseDoorLeft)
  (CallFunction|CloseDoorRight))

(event EventBeginPlay)

(fn ConstructionScript)
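; Room manager that streams connected rooms in and out as the player moves through the level.
; When a player enters its trigger, it animates a door, waits, unloads the rooms it came from except the current one, then spawns exit rooms.
; Exit levels are shuffled, streamed in and sent exit anchor transforms for entrance alignment.
; The connected-room list is then passed to each new room for later unloading.
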(event OnComponentBeginOverlap(EnteredTrigger)
  (params (OverlappedComponent :type Primitive%20Component%20Object%20Reference) (OtherActor :type Actor%20Object%20Reference) (OtherComp :type Primitive%20Component%20Object%20Reference) (OtherBodyIndex :type Integer) (bFromSweep :type Boolean) (SweepResult :type Hit%20Result%20Structure%20%28by%20ref%29))
  (if (Utilities|DoesObjectImplementInterface OtherActor "/Game/Blueprints/Interfaces/BPI_Player.BPI_Player_C")
    (Default|AnimateDoors (Variables|Default|GetDoorToClose))
    (Utilities|FlowControl|Delay 2.0)
    (Variables|Default|SetUnloadingLevelsLoopCount 0)
    (if (!= (Utilities|Array|Get(acopy) (Variables|Default|GetRoomsCameFrom) (Variables|Default|GetUnloadingLevelsLoopCount)) (Variables|Default|GetCurrentRoom)) :!label _label
      (Game|UnloadStreamLevel(byName) (Utilities|Array|Get(acopy) (Variables|Default|GetRoomsCameFrom) (Variables|Default|GetUnloadingLevelsLoopCount)) false))
    (if (== (Variables|Default|GetUnloadingLevelsLoopCount) (- (Utilities|Array|Length (Variables|Default|GetRoomsCameFrom)) 1))
      (CallFunction|SpawnExitRooms)
      (else
        (Variables|Default|SetUnloadingLevelsLoopCount (+ (Variables|Default|GetUnloadingLevelsLoopCount) 1))
        (goto _label)))))

(event Custom|SpawnExitRooms
  (bind _spawnablerooms (Variables|Default|GetSpawnableRooms))
  (if (not (Variables|Default|GetHasSpawnedExitRooms))
    (Utilities|Array|Clear (Variables|Default|GetConnectedRooms))
    (Utilities|Array|Clear _spawnablerooms)
    (Utilities|Array|AppendArray _spawnablerooms (Variables|Default|GetExitLevels))
    (Utilities|Array|Shuffle (Variables|Default|GetSpawnableRooms))
    (Game|LoadStreamLevel(byName) (CallFunction|RoomtoSpawn) true)
    (Class|BPIRoomFunctions|AlignEntrancetoExit(Message) (Class|GameplayStatics|GetStreamingLevel (CallFunction|RoomtoSpawn)) (Transformation|GetActorTransform (Utilities|Array|Get(acopy) (Variables|Default|GetExitAnchors) (Variables|Default|GetLoadingLevelsLoopCount))) :!label _label)
    (Utilities|Array|Add (Variables|Default|GetConnectedRooms) (CallFunction|RoomtoSpawn))
    (Utilities|Array|RemoveItem (Variables|Default|GetSpawnableRooms) (CallFunction|RoomtoSpawn))
    (if (== (Variables|Default|GetLoadingLevelsLoopCount) (- (Utilities|Array|Length (Variables|Default|GetExitAnchors)) 1))
      (Variables|Default|SetHasSpawnedExitRooms true)
      (CallFunction|PassConnectedRoomstoNewRooms)
      (else
        (Variables|Default|SetLoadingLevelsLoopCount (+ (Variables|Default|GetLoadingLevelsLoopCount) 1))
        (goto _label)))))

(event Custom|SetRoomsCameFrom
  (params (RoomsCameFrom :type Array%20of%20Names) (CurrentRoom :type Name) (PreviousRoom :type Name%20%28by%20ref%29))
  (bind _output_get (Variables|Default|SetRoomsCameFrom RoomsCameFrom))
  (Variables|Default|SetCurrentRoom CurrentRoom)
  (Utilities|Array|Add _output_get PreviousRoom))

(event Custom|PassConnectedRoomsToNewRooms
  (for _array_element (Variables|Default|GetConnectedRooms)
    (Class|BPIRoomFunctions|PassConnectedRooms(Message) (Class|GameplayStatics|GetStreamingLevel _array_element) (Variables|Default|GetConnectedRooms) _array_element (Variables|Default|GetCurrentRoom))))

(event EventBeginPlay)

(event Collision|EventActorBeginOverlap
  (params (OtherActor :type Actor%20Object%20Reference)))

(event EventTick
  (params (DeltaSeconds :type Float%20%28single-precision%29)))

(event EventAlignEntrancetoExit
  (params (ExitAnchor :type Transform))
  (if (!= (Variables|Default|GetEntranceAnchor) 0)
    (if (Variables|Default|GetHasAlignedEntranceToExit)
      (bind _returnvalue (Transformation|SetActorTransform (Variables|Default|GetEntranceAnchor) ExitAnchor))
      (Variables|Default|SetHasAlignedEntranceToExit _returnvalue))))

(fn ConstructionScript)

(fn RoomtoSpawn
  (return (Utilities|Array|Get(acopy) (Variables|Default|GetSpawnableRooms) (Variables|Default|GetLoadingLevelsLoopCount))))

(fn PassConnectedRooms
  (params (ConnectedRooms :type Array%20of%20Names) (CurrentRoom :type Name :default "None") (PreviousRoom :type Name :default "None"))
  (return))
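; Lightning area-of-effect ultimate spell actor that damages enemies and removes itself after a short lifetime.
; It registers as the Niagara callback and spawns a lightning strike system at each exported particle position, offset by the actor's location.
; Enemies that begin overlapping the sphere take damage through their combat component, credited to the first player.
; The overlap also reports an AI damage-sense event, with a lower amount than the damage dealt.
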(event OnComponentBeginOverlap(Sphere)
  (params (OverlappedComponent :type Primitive%20Component%20Object%20Reference) (OtherActor :type Actor%20Object%20Reference) (OtherComp :type Primitive%20Component%20Object%20Reference) (OtherBodyIndex :type Integer) (bFromSweep :type Boolean) (SweepResult :type Hit%20Result%20Structure%20%28by%20ref%29))
  (bind _asbp_enemy_base (Utilities|Casting|CastToBP_EnemyBase OtherActor))
  (Default|DamageTaken (Variables|/Game/AIStuff/AI/Enemies/BP_EnemyBase.BP_EnemyBase_C|GetBPC_Combat _asbp_enemy_base) _asbp_enemy_base 1e+02 0 (Game|GetPlayerController 0) (Game|GetPlayerCharacter 0))
  (Class|AISenseDamage|ReportDamageEvent _asbp_enemy_base (Game|GetPlayerController 0) 4e+01 (Transformation|GetActorLocation _asbp_enemy_base) "0, 0, 0" "None"))

(event EventBeginPlay
  (Niagara|SetNiagaraVariable(Object) (Variables|Default|GetNiagara) "User.BPCallBack" self)
  (Utilities|FlowControl|Delay 2.0)
  (Actor|DestroyActor))

(event EventParticleData
  (params (Data :type Array%20of%20Basic%20Particle%20Data%20Structures) (NiagaraSystem :type Niagara%20System%20Object%20Reference) (SimulationPositionOffset :type Vector%20%28by%20ref%29 :default "0, 0, 0"))
  (for _array_element Data
    (Niagara|SpawnSystematLocation "/Game/WizardSpellsPack/Effects/NS_Lightning_strike_2.NS_Lightning_strike_2" (+ (.Position (Utilities|Struct|BreakBasicParticleData _array_element)) (Transformation|GetActorLocation)))))

(fn ConstructionScript)